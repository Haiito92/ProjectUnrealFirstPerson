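; BP_PlayerGroundDisplay is a prop with a floor mesh whose center material switches between an active and inactive look.
; The construction script assigns the center material to the floor's second slot, and BeginPlay turns it into a dynamic instance, starting deactivated.
; Activate and deactivate custom events toggle that instance's StaticLightLerp scalar fully on or off.
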(event Custom|CE_Deactivate
  (Rendering|Material|SetScalarParameterValue (Variables|Default|GetCenterMatInstance) "StaticLightLerp" 0.0 :!class /Script/Engine.MaterialInstanceDynamic))

(event Custom|CE_Activate
  (Rendering|Material|SetScalarParameterValue (Variables|Default|GetCenterMatInstance) "StaticLightLerp" 1.0 :!class /Script/Engine.MaterialInstanceDynamic))

(event EventBeginPlay
  (bind _returnvalue (Rendering|Material|CreateDynamicMaterialInstance (Variables|Default|Getfloor) 1 (Variables|Default|GetCenterMaterial) "None" :!class /Script/Engine.PrimitiveComponent))
  (Variables|Default|SetCenterMatInstance _returnvalue)
  (CallFunction|CEDeactivate))

(fn ConstructionScript
  (Rendering|Material|SetMaterial (Variables|Default|Getfloor) 1 (Variables|Default|GetCenterMaterial)))