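; Spline-based wall prop that builds a wall of deformed meshes along its spline in the construction script.
; It places a start cap, repeats a loop mesh sized by its X length with the last section shortened to fit, then adds an end cap.
; Splines too short for both caps split their length proportionally between the start and end meshes.
; Each spline mesh component gets collision, Visibility blocking and custom depth rendering.
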(event EventBeginPlay)

(event Collision|EventActorBeginOverlap
  (params (OtherActor :type Actor%20Object%20Reference)))

(event EventTick
  (params (DeltaSeconds :type Float%20%28single-precision%29)))

(fn ConstructionScript
  (LocalVariables|SetStartXLength (Utilities|GetMeshXLength (Variables|Default|GetStartMesh)))
  (LocalVariables|SetEndXLength (Utilities|GetMeshXLength (Variables|Default|GetEndMesh)))
  (if (> (Spline|GetSplineLength (Variables|Default|GetSpline)) (+ (LocalVariables|GetStartXLength) (LocalVariables|GetEndXLength)))
    (LocalVariables|SetSectionLength (Utilities|GetMeshXLength (Variables|Default|GetLoopMesh)))
    (Utilities|CreateSplineMesh (Variables|Default|GetStartMesh) (.StartPos (Utilities|GetSplineSegmentPositionInfo 0.0 (LocalVariables|GetStartXLength))) (.StartTangent (Utilities|GetSplineSegmentPositionInfo 0.0 (LocalVariables|GetStartXLength))) (.EndPos (Utilities|GetSplineSegmentPositionInfo 0.0 (LocalVariables|GetStartXLength))) (.EndTangent (Utilities|GetSplineSegmentPositionInfo 0.0 (LocalVariables|GetStartXLength))))
    (LocalVariables|SetSegmentLength (LocalVariables|GetStartXLength))
    (for _index (range 0 (Math|Float|Truncate (/ (- (Spline|GetSplineLength (Variables|Default|GetSpline)) (+ (LocalVariables|GetStartXLength) (LocalVariables|GetEndXLength))) (LocalVariables|GetSectionLength))))
      (LocalVariables|SetSectionLength (Math|Float|Min(Float) (Utilities|Operators|Subtract (Spline|GetSplineLength (Variables|Default|GetSpline)) (LocalVariables|GetSegmentLength) (LocalVariables|GetEndXLength)) (LocalVariables|GetSectionLength)))
      (Utilities|CreateSplineMesh (Variables|Default|GetLoopMesh) (.StartPos (Utilities|GetSplineSegmentPositionInfo (LocalVariables|GetSegmentLength) (LocalVariables|GetSectionLength))) (.StartTangent (Utilities|GetSplineSegmentPositionInfo (LocalVariables|GetSegmentLength) (LocalVariables|GetSectionLength))) (.EndPos (Utilities|GetSplineSegmentPositionInfo (LocalVariables|GetSegmentLength) (LocalVariables|GetSectionLength))) (.EndTangent (Utilities|GetSplineSegmentPositionInfo (LocalVariables|GetSegmentLength) (LocalVariables|GetSectionLength))))
      (LocalVariables|SetSegmentLength (+ (LocalVariables|GetSectionLength) (LocalVariables|GetSegmentLength))))
    (Utilities|CreateSplineMesh (Variables|Default|GetEndMesh) (.StartPos (Utilities|GetSplineSegmentPositionInfo (LocalVariables|GetSegmentLength) (LocalVariables|GetEndXLength))) (.StartTangent (Utilities|GetSplineSegmentPositionInfo (LocalVariables|GetSegmentLength) (LocalVariables|GetEndXLength))) (.EndPos (Utilities|GetSplineSegmentPositionInfo (LocalVariables|GetSegmentLength) (LocalVariables|GetEndXLength))) (.EndTangent (Utilities|GetSplineSegmentPositionInfo (LocalVariables|GetSegmentLength) (LocalVariables|GetEndXLength))))
    (else
      (LocalVariables|SetSectionLength (* (/ (LocalVariables|GetStartXLength) (+ (LocalVariables|GetStartXLength) (LocalVariables|GetEndXLength))) (Spline|GetSplineLength (Variables|Default|GetSpline))))
      (Utilities|CreateSplineMesh (Variables|Default|GetStartMesh) (.StartPos (Utilities|GetSplineSegmentPositionInfo 0.0 (LocalVariables|GetSectionLength))) (.StartTangent (Utilities|GetSplineSegmentPositionInfo 0.0 (LocalVariables|GetSectionLength))) (.EndPos (Utilities|GetSplineSegmentPositionInfo 0.0 (LocalVariables|GetSectionLength))) (.EndTangent (Utilities|GetSplineSegmentPositionInfo 0.0 (LocalVariables|GetSectionLength))))
      (Utilities|CreateSplineMesh (Variables|Default|GetEndMesh) (.StartPos (Utilities|GetSplineSegmentPositionInfo (LocalVariables|GetSectionLength) (- (Spline|GetSplineLength (Variables|Default|GetSpline)) (LocalVariables|GetSectionLength)))) (.StartTangent (Utilities|GetSplineSegmentPositionInfo (LocalVariables|GetSectionLength) (- (Spline|GetSplineLength (Variables|Default|GetSpline)) (LocalVariables|GetSectionLength)))) (.EndPos (Utilities|GetSplineSegmentPositionInfo (LocalVariables|GetSectionLength) (- (Spline|GetSplineLength (Variables|Default|GetSpline)) (LocalVariables|GetSectionLength)))) (.EndTangent (Utilities|GetSplineSegmentPositionInfo (LocalVariables|GetSectionLength) (- (Spline|GetSplineLength (Variables|Default|GetSpline)) (LocalVariables|GetSectionLength))))))))