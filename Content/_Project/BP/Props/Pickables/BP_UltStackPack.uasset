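; BP_UltStackPack is a pickup orb that calls AddUltStack on the spell casting component of an overlapping BP_ApexCharacter.
; When that call returns false, it signals the pickup, disables sphere collision and gives the orb Niagara effect a dynamic material.
; A SphereShrink timeline then fades and dissolves the orb, scales down the platform effect and destroys the actor.
; A DoHeal function for flat or percent healing exists but is not called here.
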(event OnComponentBeginOverlap(Sphere)
  (params (OverlappedComponent :type Primitive%20Component%20Object%20Reference) (OtherActor :type Actor%20Object%20Reference) (OtherComp :type Primitive%20Component%20Object%20Reference) (OtherBodyIndex :type Integer) (bFromSweep :type Boolean) (SweepResult :type Hit%20Result%20Structure%20%28by%20ref%29))
  (bind _asbp_apex_character (Utilities|Casting|CastToBP_ApexCharacter OtherActor))
  (bind _ismax (Default|AddUltStack (Variables|/Game/_Project/BP/BP_ApexCharacter.BP_ApexCharacter_C|GetSpellCastingComponent _asbp_apex_character)))
  (if (not _ismax)
    (Default|CallItemPickedUp)
    (Collision|SetCollisionEnabled (Variables|Default|GetSphere) "NoCollision")
    (bind _returnvalue (Rendering|Material|CreateDynamicMaterialInstance "/Game/_Project/Assets/Materials/FX/UltOrb/M_UltOrb_InstDeTesMorts.M_UltOrb_InstDeTesMorts" "Crampté" "None" :!class /Script/Engine.KismetMaterialLibrary))
    (bind _output_get (Variables|Default|SetMat _returnvalue))
    (Class|NiagaraComponent|SetVariableMaterial (Variables|Default|GetNS_UltOrb) "Mat" _output_get)
    (bind _shrink (Timeline|Sphere%20Shrink Play)
      (:Update
        (Rendering|Material|SetScalarParameterValue (Variables|Default|GetMat) "Fade" (Math|Float|Lerp 1.0 0.0 _shrink) :!class /Script/Engine.MaterialInstanceDynamic)
        (Niagara|SetNiagaraVariable(Float) (Variables|Default|GetNS_UltOrb) "2ndMatDissolve" (Math|Float|Lerp 1.0 0.0 _shrink))
        (Niagara|SetNiagaraVariable(Float) (Variables|Default|GetNS_UltPlatform) "Scale" (Math|Float|Lerp 1.0 0.0 _shrink)))
      (:Finished
        (Actor|DestroyActor)))))

(event EventBeginPlay)

(event Collision|EventActorBeginOverlap
  (params (OtherActor :type Actor%20Object%20Reference)))

(event EventTick
  (params (DeltaSeconds :type Float%20%28single-precision%29)))

(fn ConstructionScript)

(fn DoHeal
  (params (Player :type BP%20Apex%20Character%20Object%20Reference))
  (bind _healed (Default|Heal Player (Math|Float|SelectFloat (* (Variables|Default|GetHealAmount) (Variables|/Game/_Project/Data/Blueprints/BPDA_CharacterInfo.BPDA_CharacterInfo_C|GetMaxHp (Variables|/Game/_Project/BP/BP_ApexCharacter.BP_ApexCharacter_C|GetCharacterInfo Player))) (Variables|Default|GetHealAmount) (Variables|Default|GetHealIsPercentHP))))
  (return _healed))