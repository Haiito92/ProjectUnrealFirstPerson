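; Ammo pickup prop that refills the bullets of a BP_ApexCharacter that touches it.
; Sphere overlap casts the other actor to BP_ApexCharacter and calls DoAmmoRefill, which adds bullets through its BP_Weapon_Component, as either rounds or magazines.
; On success it calls CallItemPickedUp and destroys itself; without a valid weapon component it stays in the world.
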(event OnComponentBeginOverlap(Sphere)
  (params (OverlappedComponent :type Primitive%20Component%20Object%20Reference) (OtherActor :type Actor%20Object%20Reference) (OtherComp :type Primitive%20Component%20Object%20Reference) (OtherBodyIndex :type Integer) (bFromSweep :type Boolean) (SweepResult :type Hit%20Result%20Structure%20%28by%20ref%29))
  (bind _asbp_apex_character (Utilities|Casting|CastToBP_ApexCharacter OtherActor))
  (bind _couldrefill (CallFunction|DoAmmoRefill _asbp_apex_character))
  (if _couldrefill
    (Default|CallItemPickedUp)
    (Actor|DestroyActor)))

(event EventBeginPlay)

(event Collision|EventActorBeginOverlap
  (params (OtherActor :type Actor%20Object%20Reference)))

(event EventTick
  (params (DeltaSeconds :type Float%20%28single-precision%29)))

(fn ConstructionScript)

(fn DoAmmoRefill
  (params (Player :type Actor%20Object%20Reference))
  (bind _returnvalue (Actor|GetComponentbyClass Player "/Game/_Project/BP/Components/BP_Weapon_Component.BP_Weapon_Component_C"))
  (Utilities|IsValid _returnvalue
    (:Is%20Valid
      (Default|AddBullets _returnvalue (Variables|Default|GetBulletsNumber) (Variables|Default|GetBulletsNumberIsMagNumber))
      (return true))
    (:Is%20Not%20Valid
      (return false))))