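; BP_PickableSpawner is a prop that spawns a pickable item above itself, immediately or after a random delay.
; Each item's pickup event plays a sound and schedules a randomly timed respawn while spawns remain, with a maximum of -1 meaning unlimited.
; Spawning and pickup trigger a Tick-driven lerp of a dynamic material parameter on the floor's center, swapping its light color to show item availability.
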(event Custom|CE_SpawnItem
  (bind _returnvalue (Transformation|GetActorTransform))
  (Utilities|FlowControl|Sequence
    (:then_0
      (CallFunction|DoColorSwap 1.0))
    (:then_1
      (bind _returnvalue_2 (Game|SpawnActorfromClass (Variables|Default|GetClassToSpawn) (Math|Transform|MakeTransform (+ (.location _returnvalue) (Math|Vector|MakeVector 0.0 0.0 (Variables|Default|GetSpawnZOffset))) (.rotation _returnvalue) (.scale _returnvalue)) "AlwaysSpawn" "MultiplyWithRoot" 0 0))
      (Math|Integer|DecrementInt (Variables|Default|GetSpawnsLeft)
        (:%20%20
          (Utilities|IsValid _returnvalue_2
            (:Is%20Valid
              (EventDispatchers|AssignItemPickedUp _returnvalue_2 (delegate Custom|CE_OnSpawnedItemPickedUp)))
            (:Is%20Not%20Valid
              (CallFunction|CEonSpawnedItemPickedUp))))))))

(event Custom|CE_OnSpawnedItemPickedUp
  ;[1 1 1] On Item Pickup we try to start the respawn timer
  (Audio|PlaySoundatLocation (Variables|Sound|GetPickedUpSound) (Transformation|GetActorLocation) "0, 0, 0" 1.0 1.0 0.0 0 0 0 0)
  (CallFunction|DoColorSwap 0.0)
  (if (Utilities|CanSpawnItem)
    (Utilities|Time|SetTimerbyEvent (EventDispatchers|CreateEvent :!event Custom|CE_SpawnItem) (Math|Random|RandomFloatinRange (Variables|Default|GetMinRandomSpawnTime) (Variables|Default|GetMaxRandomSpawnTime)))))

(event Custom|DoColorSwap
  (params (TargetLerpVal :type Float%20%28double-precision%29))
  (Variables|ColorSwap|SetTargetLerpVal TargetLerpVal)
  (Variables|ColorSwap|SetIsColorSwapping true)
  (Variables|ColorSwap|SetLerpDelta 0.0))

(event EventBeginPlay
  (Variables|Default|SetSpawnsLeft (Variables|Default|GetMaxNumberOfSpawns))
  (bind _returnvalue (Rendering|Material|CreateDynamicMaterialInstance (Variables|Default|Getfloor) 1 (Variables|Default|GetCenterMaterial) "None" :!class /Script/Engine.PrimitiveComponent))
  (Variables|Default|SetCenterMatInstance _returnvalue)
  ;[1 1 1] Spawn Item Immediatly or start random respawn timer
  (if (and (Variables|Default|GetSpawnOnBeginPlay) (Utilities|CanSpawnItem))
    (CallFunction|CESpawnItem)
    (else
      (Utilities|Time|SetTimerbyEvent (EventDispatchers|CreateEvent :!event Custom|CE_SpawnItem) (Math|Random|RandomFloatinRange (Variables|Default|GetMinRandomSpawnTime) (Variables|Default|GetMaxRandomSpawnTime))))))

(event EventTick
  (params (DeltaSeconds :type Float%20%28single-precision%29))
  (if (Variables|ColorSwap|GetIsColorSwapping)
    (bind _output_get (Variables|ColorSwap|SetLerpDelta (+ DeltaSeconds (Variables|ColorSwap|GetLerpDelta))))
    (Rendering|Material|SetScalarParameterValue (Variables|Default|GetCenterMatInstance) "StaticLightLerp" (|GetLerpValue _output_get) :!class /Script/Engine.MaterialInstanceDynamic)))

(fn ConstructionScript
  (Rendering|Material|SetMaterial (Variables|Default|Getfloor) 1 (Variables|Default|GetCenterMaterial)))