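; BP_HealthPack is a pickup prop that heals the player character on contact.
; A sphere overlap with BP_ApexCharacter calls DoHeal, which passes either a flat HealAmount or a percentage of max HP to the character, depending on HealIsPercentHP.
; It then calls ItemPickedUp and destroys itself, regardless of the returned heal result.
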(event OnComponentBeginOverlap(Sphere)
  (params (OverlappedComponent :type Primitive%20Component%20Object%20Reference) (OtherActor :type Actor%20Object%20Reference) (OtherComp :type Primitive%20Component%20Object%20Reference) (OtherBodyIndex :type Integer) (bFromSweep :type Boolean) (SweepResult :type Hit%20Result%20Structure%20%28by%20ref%29))
  (bind _asbp_apex_character (Utilities|Casting|CastToBP_ApexCharacter OtherActor))
  (bind _healed (CallFunction|DoHeal _asbp_apex_character))
  (if _healed
    _
    (else
      _))
  (Default|CallItemPickedUp)
  (Actor|DestroyActor))

(event EventBeginPlay)

(event Collision|EventActorBeginOverlap
  (params (OtherActor :type Actor%20Object%20Reference)))

(event EventTick
  (params (DeltaSeconds :type Float%20%28single-precision%29)))

(fn ConstructionScript)

(fn DoHeal
  (params (Player :type IN%20Damageable%20Interface))
  (bind _maxhp (Default|GetMaxHP Player))
  (bind _healed (Default|DoHeal Player (Math|Float|SelectFloat (* _maxhp (/ (Variables|Default|GetHealAmount) 1e+02)) (Variables|Default|GetHealAmount) (Variables|Default|GetHealIsPercentHP))))
  (return _healed))