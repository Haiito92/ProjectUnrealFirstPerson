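; Deathmatch game mode for local multiplayer that ends on a kill target or time limit, depending on the configured mode.
; Spawns and possesses a character per local player, then checks the win condition on deaths or timer ticks.
; Dead players respawn after a delay at random, preferably enabled points, keeping ult charges, while old bodies remain as capped ragdolls.
; Game end triggers time dilation; score and winner feed Discord presence.
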(event Custom|CE_DoTimer
  ;[1 1 1] Increment Timer and check if over
  (if (not (Variables|Default|GetIsOver))
    (bind _result (Math|Integer|IncrementInt (Variables|Default|GetTimer))
      (:%20%20
        (if (>= _result (.timeramount (Variables|/Game/_Project/BP/BP_ApexGameInstance.BP_ApexGameInstance_C|GetDeathMatchInfo (Variables|Default|GetGameInstance))))
          (bind _playerindex (CallFunction|FindPlayerwithMostKills))
          (CallFunction|CEEndGame _playerindex))))))

(event Custom|CE_DoDelayedRespawn
  (params (PlayerDead :type BP%20Apex%20Character%20Object%20Reference))
  (Utilities|FlowControl|Delay (Variables|Default|GetTimeBeforeRespawn))
  (Widget|RemovefromParent (Variables|/Game/_Project/BP/BP_ApexCharacter.BP_ApexCharacter_C|GetGUI PlayerDead))
  (CallFunction|RespawnPlayer (Utilities|Struct|MakeST_PlayerRespawnInfo (Variables|/Game/_Project/BP/BP_ApexCharacter.BP_ApexCharacter_C|GetPlayerIndex PlayerDead) (Variables|/Game/_Project/BP/BP_ApexCharacter.BP_ApexCharacter_C|GetCharacterInfo PlayerDead) (Variables|/Game/_Project/BP/BP_SpellCastingComponent.BP_SpellCastingComponent_C|GetUltStack (Variables|/Game/_Project/BP/BP_ApexCharacter.BP_ApexCharacter_C|GetSpellCastingComponent PlayerDead))))
  (CallFunction|AddRagdoll PlayerDead))

(event Custom|CE_PlayerDeath
  (params (Killer :type BP%20Apex%20Character%20Object%20Reference) (PlayerDead :type BP%20Apex%20Character%20Object%20Reference))
  ;[1 1 1] Logic called when a Player is killed
  (CallFunction|PlayerDeathFunc Killer PlayerDead)
  (CallFunction|UpdateDiscordRP))

(event Custom|CE_EndGame
  (params (WinnerPlayerIndex :type Integer))
  (CallFunction|EndGame WinnerPlayerIndex))

(event Custom|CE_Update
  (Class|DiscordGameInstance|SetDiscordPresencewithTimestampOption (Variables|Default|GetGameInstance) "Update" false))

(event EventBeginPlay
  (|CallParentFunction)
  (Utilities|FlowControl|Sequence
    (:then_0
      (if (Utilities|Enum|NotEqual(Enum) (Utilities|GetDeathmatchMode) "NewEnumerator0")
        (Utilities|Time|SetTimerbyEvent (EventDispatchers|CreateEvent :!event Custom|CE_DoTimer) 1.0 true)))
    (:then_1
      (bind _returnvalue (Game|SpawnActorfromClass "/Game/_Project/BP/Lvl0/BP_TimeDilator.BP_TimeDilator_C" (Math|Transform|MakeTransform "0, 0, 0" "0, 0, 0" "1.000000,1.000000,1.000000") "Undefined" "MultiplyWithRoot" 0 0))
      (Variables|Default|SetTimeDilator _returnvalue)
      (CallFunction|UpdateDiscordRP)
      (Class|DiscordGameInstance|SetDiscordPresencewithTimestampOption (Variables|Default|GetGameInstance) "Update" true))))

(fn ConstructionScript)

(fn IsGameOverKills
  (bind _values (Utilities|Map|Values (Variables|Default|GetPlayerScores)))
  (for (_array_element _array_index) _values
    (if (>= (Utilities|Struct|BreakST_PlayerScore _array_element) (.requiredkillsamount (Variables|/Game/_Project/BP/BP_ApexGameInstance.BP_ApexGameInstance_C|GetDeathMatchInfo (Variables|Default|GetGameInstance))))
      (return true _array_index)))
  (return false 0))

(fn FindPlayerwithMostKills
  (bind _values (Utilities|Map|Values (Variables|Default|GetPlayerScores)))
  (for (_array_element _array_index) _values
    (if (> (Utilities|Struct|BreakST_PlayerScore _array_element) (LocalVariables|GetLastKillNumber))
      (LocalVariables|SetLastKillNumber (Utilities|Struct|BreakST_PlayerScore _array_element))
      (LocalVariables|SetPlayerID _array_index)))
  (return (LocalVariables|GetPlayerID)))

(fn SpawnPlayers
  (params (PlayerCount :type Integer))
  (bind _outactors (Actor|GetAllActorsOfClass "/Script/Engine.PlayerStart"))
  (bind (_array_element _array_index) (Utilities|Array|ForEachLoopwithBreak _outactors :!label _label)
    (:LoopBody
      (if (< _array_index PlayerCount)
        (bind _output_get (LocalVariables|SetArray%20Index _array_index))
        (bind _returnvalue (Class|GameplayStatics|CreatePlayer _output_get)) ; Create local player controller
        (Input|AddMappingContext (PlayerController|LocalPlayerSubsystems|GetEnhancedInputLocalPlayerSubsystem (select (== (LocalVariables|GetArray%20Index) 0) (Game|GetPlayerController 0) _returnvalue)) "/Game/_Project/Input/IMC_Default.IMC_Default" 0 "(bIgnoreAllPressedKeysUntilRelease=True,bForceImmediately=False,bNotifyUserSettings=False)") ; Assign the input mapping to the player
        (bind _returnvalue_2 (Game|SpawnActorfromClass "/Game/_Project/BP/BP_ApexCharacter.BP_ApexCharacter_C" (Transformation|GetActorTransform _array_element) "Undefined" "MultiplyWithRoot" 0 (.Value (Utilities|Map|Find (Variables|/Game/_Project/BP/BP_ApexGameInstance.BP_ApexGameInstance_C|GetPlayerCharacterMap (Variables|Default|GetGameInstance)) (LocalVariables|GetArray%20Index))) (LocalVariables|GetArray%20Index) 0))
        (Pawn|Possess (Game|GetPlayerController (LocalVariables|GetArray%20Index)) _returnvalue_2) ; Assign controller to player
        (Utilities|Map|Add (Variables|Default|GetPlayerScores) (|Copy (LocalVariables|GetArray%20Index)) (|Copy (Utilities|Struct|MakeST_PlayerScore)))
        (else
          (goto _label Break))))
    (:Completed
      (for _index (range 0 _array_index)
        _))))

(fn AddRagdoll
  (params (Player%20Ragdoll :type BP%20Apex%20Character%20Object%20Reference%20%28by%20ref%29))
  (bind _ragdolls (Variables|Default|GetRagdolls))
  (if (>= (Utilities|Array|Length (Variables|Default|GetRagdolls)) (Variables|Default|GetMaxRagdolls))
    (Actor|DestroyActor (Utilities|Array|Get(acopy) _ragdolls))
    (Utilities|Array|RemoveIndex _ragdolls))
  (Utilities|Array|Add (Variables|Default|GetRagdolls) Player%20Ragdoll))

(fn PlayerDeathFunc
  (params (Killer :type BP%20Apex%20Character%20Object%20Reference) (PlayerDead :type BP%20Apex%20Character%20Object%20Reference))
  (if (not (Variables|Default|GetIsOver))
    (|CallParentFunction Killer PlayerDead)
    (Default|Kill PlayerDead)
    (if (Utilities|Enum|NotEqual(Enum) (Utilities|GetDeathmatchMode) "NewEnumerator1")
      (bind (_state _winnerplayerindex) (CallFunction|IsGameOverKills))
      (if _state
        (CallFunction|CEEndGame _winnerplayerindex)
        (else
          (CallFunction|CEDoDelayedRespawn PlayerDead :!label _label)))
      (else
        (goto _label)))))

(fn EndGame
  (params (WinnerPlayerIndex :type Integer))
  (bind _gameinstance (Variables|Default|GetGameInstance))
  (if (not (Variables|Default|GetIsOver))
    (|CallParentFunction WinnerPlayerIndex)
    (Default|CEEndGameTimeDilation (Variables|Default|GetTimeDilator))
    (Class|DiscordGameInstance|SetBasicPresence _gameinstance (Utilities|String|BuildString(Integer) "" "Player " WinnerPlayerIndex " Won!") "In Deathmatch")
    (Class|DiscordGameInstance|SetDiscordPresencewithTimestampOption _gameinstance "Update" false)))

(fn UpdateDiscordRP
  (bind _playerscores (Variables|Default|GetPlayerScores))
  (Class|DiscordGameInstance|SetBasicPresence (Variables|Default|GetGameInstance) (Utilities|String|Append (Utilities|String|ToString(Integer) (.Kills (Utilities|Struct|BreakST_PlayerScore (.Value (Utilities|Map|Find _playerscores 0))))) " - " (Utilities|String|ToString(Integer) (.Kills (Utilities|Struct|BreakST_PlayerScore (.Value (Utilities|Map|Find _playerscores 1)))))) "In DeathMatch"))

(fn RespawnPlayer
  (params (PlayerRespawnInfo :type ST%20Player%20Respawn%20Info%20Structure))
  (bind _playerindex (Utilities|Struct|BreakST_PlayerRespawnInfo PlayerRespawnInfo))
  (bind _returnvalue (Game|GetPlayerController _playerindex))
  (bind _output_get (LocalVariables|SetSpawnPoint (.OutItem (Utilities|Array|Random (Variables|Default|GetRespawnPoints)))))
  (while (and (Default|IsDisabled _output_get) (< (LocalVariables|GetLoopIterations) 50))
    ;[1 1 1] Try to get a spawn point that is not disabled, else go brrr
    (LocalVariables|SetSpawnPoint (.OutItem (Utilities|Array|Random (Variables|Default|GetRespawnPoints))))
    (Math|Integer|IncrementInt (LocalVariables|GetLoopIterations)))
  (bind _returnvalue_2 (Game|SpawnActorfromClass "/Game/_Project/BP/BP_ApexCharacter.BP_ApexCharacter_C" (Math|Transform|MakeTransform (+ (.location (Transformation|GetActorTransform (LocalVariables|GetSpawnPoint))) "0.000000,0.000000,96.000000") (.rotation (Transformation|GetActorTransform (LocalVariables|GetSpawnPoint))) (.scale (Transformation|GetActorTransform (LocalVariables|GetSpawnPoint)))) "AlwaysSpawn" "MultiplyWithRoot" 0 (.characterinfo PlayerRespawnInfo) (.playerindex PlayerRespawnInfo) 0))
  (Pawn|Possess _returnvalue _returnvalue_2) ; Assign controller to player
  (Variables|/Game/_Project/BP/BP_SpellCastingComponent.BP_SpellCastingComponent_C|SetUltStack (Variables|/Game/_Project/BP/BP_ApexCharacter.BP_ApexCharacter_C|GetSpellCastingComponent _returnvalue_2) (.ultcharges PlayerRespawnInfo))
  (Default|CallPlayerRespawn _returnvalue_2)
  (bind _asbp_apex_player_controller (Utilities|Casting|CastToBP_ApexPlayerController _returnvalue))
  (Default|OnPlayerRespawn _asbp_apex_player_controller))