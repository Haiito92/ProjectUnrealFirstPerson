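; Practice-mode game mode that spawns local players, respawns them after death and shows practice status in Discord Rich Presence.
; SpawnPlayers creates controllers and possesses BP_ApexCharacters at PlayerStarts.
; Deaths trigger a delayed respawn at a random RespawnPoint, retrying disabled ones up to a loop limit, then destroy the old pawn.
; It also caps ragdolls by removing the oldest, and EndGame triggers time dilation and a winner presence labelled Deathmatch.
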(event Custom|CE_DoDelayedRespawn
  (params (PlayerDead :type BP%20Apex%20Character%20Object%20Reference))
  (Utilities|FlowControl|Delay (Variables|Default|GetTimeBeforeRespawn))
  (CallFunction|RespawnPlayer (Utilities|Struct|MakeST_PlayerRespawnInfo (Variables|/Game/_Project/BP/BP_ApexCharacter.BP_ApexCharacter_C|GetPlayerIndex PlayerDead) (Variables|/Game/_Project/BP/BP_ApexCharacter.BP_ApexCharacter_C|GetCharacterInfo PlayerDead) (Variables|/Game/_Project/BP/BP_SpellCastingComponent.BP_SpellCastingComponent_C|GetUltStack (Variables|/Game/_Project/BP/BP_ApexCharacter.BP_ApexCharacter_C|GetSpellCastingComponent PlayerDead))))
  (Actor|DestroyActor PlayerDead))

(event Custom|CE_PlayerDeath
  (params (Killer :type BP%20Apex%20Character%20Object%20Reference) (PlayerDead :type BP%20Apex%20Character%20Object%20Reference))
  ;[1 1 1] Logic called when a Player is killed
  (CallFunction|PlayerDeathFunc Killer PlayerDead)
  (CallFunction|UpdateDiscordRP))

(event Custom|CE_EndGame
  (params (WinnerPlayerIndex :type Integer))
  (CallFunction|EndGame WinnerPlayerIndex))

(event EventBeginPlay
  (|CallParentFunction)
  (Utilities|FlowControl|Sequence
    (:then_1
      (CallFunction|UpdateDiscordRP)
      (Class|DiscordGameInstance|SetDiscordPresencewithTimestampOption (Variables|Default|GetGameInstance) "Update" true))))

(fn ConstructionScript)

(fn SpawnPlayers
  (params (PlayerCount :type Integer))
  (bind _outactors (Actor|GetAllActorsOfClass "/Script/Engine.PlayerStart"))
  (bind (_array_element _array_index) (Utilities|Array|ForEachLoopwithBreak _outactors :!label _label)
    (:LoopBody
      (if (< _array_index PlayerCount)
        (bind _output_get (LocalVariables|SetArray%20Index _array_index))
        (bind _returnvalue (Class|GameplayStatics|CreatePlayer _output_get)) ; Create local player controller
        (Input|AddMappingContext (PlayerController|LocalPlayerSubsystems|GetEnhancedInputLocalPlayerSubsystem (select (== (LocalVariables|GetArray%20Index) 0) (Game|GetPlayerController 0) _returnvalue)) "/Game/_Project/Input/IMC_Default.IMC_Default" 0 "(bIgnoreAllPressedKeysUntilRelease=True,bForceImmediately=False,bNotifyUserSettings=False)") ; Assign the input mapping to the player
        (bind _returnvalue_2 (Game|SpawnActorfromClass "/Game/_Project/BP/BP_ApexCharacter.BP_ApexCharacter_C" (Transformation|GetActorTransform _array_element) "Undefined" "MultiplyWithRoot" 0 (.Value (Utilities|Map|Find (Variables|/Game/_Project/BP/BP_ApexGameInstance.BP_ApexGameInstance_C|GetPlayerCharacterMap (Variables|Default|GetGameInstance)) (LocalVariables|GetArray%20Index))) (LocalVariables|GetArray%20Index) 0))
        (Pawn|Possess (Game|GetPlayerController (LocalVariables|GetArray%20Index)) _returnvalue_2) ; Assign controller to player
        (Utilities|Map|Add (Variables|Default|GetPlayerScores) (|Copy (LocalVariables|GetArray%20Index)) (|Copy (Utilities|Struct|MakeST_PlayerScore)))
        (else
          (goto _label Break))))
    (:Completed
      (for _index (range 0 _array_index)
        _))))

(fn RespawnPlayer
  (params (RespawnInfo :type ST%20Player%20Respawn%20Info%20Structure))
  (bind _playerindex (Utilities|Struct|BreakST_PlayerRespawnInfo RespawnInfo))
  (bind _returnvalue (Game|GetPlayerController _playerindex))
  (bind _output_get (LocalVariables|SetSpawnPoint (.OutItem (Utilities|Array|Random (Variables|Default|GetRespawnPoints)))))
  (while (and (Default|IsDisabled _output_get) (< (LocalVariables|GetLoopIterations) 50))
    ;[1 1 1] Try to get a spawn point that is not disabled, else go brrr
    (LocalVariables|SetSpawnPoint (.OutItem (Utilities|Array|Random (Variables|Default|GetRespawnPoints))))
    (Math|Integer|IncrementInt (LocalVariables|GetLoopIterations)))
  (bind _returnvalue_2 (Game|SpawnActorfromClass "/Game/_Project/BP/BP_ApexCharacter.BP_ApexCharacter_C" (Math|Transform|MakeTransform (+ (.location (Transformation|GetActorTransform (LocalVariables|GetSpawnPoint))) "0.000000,0.000000,96.000000") (.rotation (Transformation|GetActorTransform (LocalVariables|GetSpawnPoint))) (.scale (Transformation|GetActorTransform (LocalVariables|GetSpawnPoint)))) "AlwaysSpawn" "MultiplyWithRoot" 0 (.characterinfo RespawnInfo) (.playerindex RespawnInfo) 0))
  (Pawn|Possess _returnvalue _returnvalue_2) ; Assign controller to player
  (Default|CallPlayerRespawn _returnvalue_2)
  (bind _asbp_apex_player_controller (Utilities|Casting|CastToBP_ApexPlayerController _returnvalue))
  (Default|OnPlayerRespawn _asbp_apex_player_controller))

(fn AddRagdoll
  (params (Player%20Ragdoll :type BP%20Apex%20Character%20Object%20Reference%20%28by%20ref%29))
  (bind _ragdolls (Variables|Default|GetRagdolls))
  (if (>= (Utilities|Array|Length (Variables|Default|GetRagdolls)) (Variables|Default|GetMaxRagdolls))
    (Actor|DestroyActor (Utilities|Array|Get(acopy) _ragdolls))
    (Utilities|Array|RemoveIndex _ragdolls))
  (Utilities|Array|Add (Variables|Default|GetRagdolls) Player%20Ragdoll))

(fn PlayerDeathFunc
  (params (Killer :type BP%20Apex%20Character%20Object%20Reference) (PlayerDead :type BP%20Apex%20Character%20Object%20Reference))
  (if (not (Variables|Default|GetIsOver))
    (|CallParentFunction Killer PlayerDead)
    (Default|Kill PlayerDead)
    (CallFunction|CEDoDelayedRespawn PlayerDead)))

(fn EndGame
  (params (WinnerPlayerIndex :type Integer))
  (bind _gameinstance (Variables|Default|GetGameInstance))
  (if (not (Variables|Default|GetIsOver))
    (|CallParentFunction WinnerPlayerIndex)
    (Default|CEEndGameTimeDilation (Variables|Default|GetTimeDilator))
    (Class|DiscordGameInstance|SetBasicPresence _gameinstance (Utilities|String|BuildString(Integer) "" "Player " WinnerPlayerIndex " Won!") "In Deathmatch")
    (Class|DiscordGameInstance|SetDiscordPresencewithTimestampOption _gameinstance "Update" false)))

(fn UpdateDiscordRP
  (Class|DiscordGameInstance|SetBasicPresence (Variables|Default|GetGameInstance) "Get Good" "In Practice Mode"))