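; Base game mode for Apex that tracks per-player combat scores and announces player deaths and game end.
; BeginPlay caches the game instance, calls SpawnPlayers with its player count, then collects respawn points; spawn and respawn functions are empty here.
; Events and death handling update a score map keyed by player index until IsOver is set.
; EndGame sets that flag and broadcasts the winner with two players' kills.
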(event Custom|CE_BulletHit
  (params (PlayerIndex :type Integer) (IsHeadShot :type Boolean))
  (bind _playerscores (Variables|Default|GetPlayerScores))
  (bind _value (Utilities|Map|Find _playerscores PlayerIndex))
  (bind (_bulletshit _headshothits) (Utilities|Struct|BreakST_PlayerScore _value))
  ;[1 1 1] Player Hit another Player with a bullet
  (if (not (Variables|Default|GetIsOver))
    (bind _structout (Utilities|Struct|SetmembersinST_PlayerScore _value (+ _bulletshit 1) (+ _headshothits (Math|Integer|SelectInt 1 0 IsHeadShot))))
    (Utilities|Map|Add (Variables|Default|GetPlayerScores) PlayerIndex _structout)))

(event Custom|CE_BulletShot
  (params (PlayerIndex :type Integer))
  (bind _playerscores (Variables|Default|GetPlayerScores))
  (bind _value (Utilities|Map|Find _playerscores PlayerIndex))
  ;[1 1 1] Player Fired a bullet
  (if (not (Variables|Default|GetIsOver))
    (bind _structout (Utilities|Struct|SetmembersinST_PlayerScore _value (+ (Utilities|Struct|BreakST_PlayerScore _value) 1)))
    (Utilities|Map|Add (Variables|Default|GetPlayerScores) PlayerIndex _structout)))

(event Custom|CE_AddDamageScore
  (params (DmgDealer :type BP%20Apex%20Character%20Object%20Reference) (DmgAmount :type Float%20%28double-precision%29))
  (bind _playerscores (Variables|Default|GetPlayerScores))
  (bind _playerindex (Variables|/Game/_Project/BP/BP_ApexCharacter.BP_ApexCharacter_C|GetPlayerIndex DmgDealer))
  (bind _value (Utilities|Map|Find _playerscores _playerindex))
  ;[1 1 1] Add Damage dealt by Player to his score
  (if (not (Variables|Default|GetIsOver))
    (bind _structout (Utilities|Struct|SetmembersinST_PlayerScore _value (+ (Utilities|Struct|BreakST_PlayerScore _value) DmgAmount)))
    (Utilities|Map|Add (Variables|Default|GetPlayerScores) (Variables|/Game/_Project/BP/BP_ApexCharacter.BP_ApexCharacter_C|GetPlayerIndex DmgDealer) _structout)))

(event EventBeginPlay
  (bind _asbp_apex_game_instance (Utilities|Casting|CastToBP_ApexGameInstance (Game|GetGameInstance)))
  (bind _output_get (Variables|Default|SetGameInstance _asbp_apex_game_instance))
  (CallFunction|SpawnPlayers (Variables|/Game/_Project/BP/BP_ApexGameInstance.BP_ApexGameInstance_C|GetPlayerCount _output_get))
  (bind _outactors (Actor|GetAllActorsOfClass "/Game/_Project/BP/Lvl0/BP_RespawnPoint.BP_RespawnPoint_C"))
  (for _array_element _outactors
    (Utilities|Array|Add (Variables|Default|GetRespawnPoints) _array_element)))

(fn ConstructionScript)

(fn SpawnPlayers
  (params (PlayerCount :type Integer)))

(fn RespawnPlayer
  (params (Player%20Index :type Integer) (CharacterInfo :type BPDA%20Character%20Info%20Object%20Reference)))

(fn PlayerDeathFunc
  (params (Killer :type BP%20Apex%20Character%20Object%20Reference) (PlayerDead :type BP%20Apex%20Character%20Object%20Reference))
  (if (not (Variables|Default|GetIsOver))
    (|UpdateScores Killer PlayerDead
      (:execute
        (Default|CallPlayerDeath Killer PlayerDead)))))

(fn EndGame
  (params (WinnerPlayerIndex :type Integer))
  (bind _playerscores (Variables|Default|GetPlayerScores))
  (bind (_value _returnvalue) (Utilities|Map|Find _playerscores 0))
  (bind (_value_2 _returnvalue_2) (Utilities|Map|Find _playerscores 1))
  (if (not (Variables|Default|GetIsOver))
    (Development|PrintString (Utilities|String|BuildString(Integer) "" "Player " WinnerPlayerIndex " Won"))
    (Variables|Default|SetIsOver true)
    (Default|CallGameEnded WinnerPlayerIndex (Math|Integer|SelectInt (.Kills (Utilities|Struct|BreakST_PlayerScore _value)) 0 _returnvalue) (Math|Integer|SelectInt (.Kills (Utilities|Struct|BreakST_PlayerScore _value_2)) 0 _returnvalue_2))))