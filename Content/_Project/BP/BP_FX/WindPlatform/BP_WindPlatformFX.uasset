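; BP_WindPlatformFX is a temporary wind platform that BP_ApexCharacter can pass through from below.
; Overlapping BeneathColl with that character turns MainColl collision off, and leaving it restores query and physics collision, giving one-way platform behavior.
; After PlatformDuration it deactivates the Niagara effect, disables collision, ignores further overlaps through IsDeactivateIn, then destroys itself following a short delay.
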(event OnComponentBeginOverlap(BeneathColl)
  (params (OverlappedComponent :type Primitive%20Component%20Object%20Reference) (OtherActor :type Actor%20Object%20Reference) (OtherComp :type Primitive%20Component%20Object%20Reference) (OtherBodyIndex :type Integer) (bFromSweep :type Boolean) (SweepResult :type Hit%20Result%20Structure%20%28by%20ref%29))
  (if (not (Variables|Default|GetIsDeactivateIn))
    (Utilities|Casting|CastToBP_ApexCharacter OtherActor)
    (Collision|SetCollisionEnabled (Variables|Default|GetMainColl) "NoCollision")))

(event OnComponentEndOverlap(BeneathColl)
  (params (OverlappedComponent :type Primitive%20Component%20Object%20Reference) (OtherActor :type Actor%20Object%20Reference) (OtherComp :type Primitive%20Component%20Object%20Reference) (OtherBodyIndex :type Integer))
  (if (not (Variables|Default|GetIsDeactivateIn))
    (Utilities|Casting|CastToBP_ApexCharacter OtherActor)
    (Collision|SetCollisionEnabled (Variables|Default|GetMainColl) "QueryAndPhysics")))

(event EventBeginPlay
  (Utilities|FlowControl|Delay (Variables|Default|GetPlatformDuration))
  (Components|Activation|Deactivate (Variables|Default|GetNS_WindPlateform))
  (Variables|Default|SetIsDeactivateIn true)
  (Collision|SetCollisionEnabled (Variables|Default|GetMainColl) "NoCollision")
  (Utilities|FlowControl|Delay 5.0)
  (Actor|DestroyActor))

(fn ConstructionScript)