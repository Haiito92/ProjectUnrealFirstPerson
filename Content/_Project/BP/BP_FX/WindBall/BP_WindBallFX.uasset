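; BP_WindBallFX is a wind ball projectile that turns into a tornado when it lands on a surface.
; On a Sphere hit, it compares the normalized impulse against world up, so only near-vertical impacts trigger it.
; It then spawns BP_TornadoFX at its location with duration and push scale passed from its own variables, plays a 2D hit sound, and destroys itself.
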(event OnComponentHit(Sphere)
  (params (HitComponent :type Primitive%20Component%20Object%20Reference) (OtherActor :type Actor%20Object%20Reference) (OtherComp :type Primitive%20Component%20Object%20Reference) (NormalImpulse :type Vector :default "0, 0, 0") (Hit :type Hit%20Result%20Structure%20%28by%20ref%29))
  (if (> (Math|Vector|DotProduct "0.000000,0.000000,1.000000" (Math|Vector|Normalize NormalImpulse)) 0.9)
    (Game|SpawnActorfromClass "/Game/_Project/BP/BP_FX/WindBall/BP_TornadoFX.BP_TornadoFX_C" (Math|Transform|MakeTransform (Transformation|GetActorLocation) "0, 0, 0" "1.000000,1.000000,1.000000") "AlwaysSpawn" "MultiplyWithRoot" 0 (Variables|Default|GetMainTornadoDurationWindBall) (Variables|Default|GetMainTornadoPushScale) 0)
    ;[1 1 1] Need to be stereo (not done)
    (Audio|PlaySound2D (Variables|Default|GetHitingSound) 1.0 1.0 0.0 0 0 false)
    (Actor|DestroyActor)))

(event EventBeginPlay)

(fn ConstructionScript)