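; BP_TornadoFX is a temporary tornado effect actor that throws overlapping characters and physics objects upward.
; On box overlap it launches characters vertically, or applies a stronger velocity-change impulse to other components that simulate physics.
; After MainTornadoDuration it prints a debug string, deactivates the Niagara effect, disables box collision, and destroys itself following a short delay.
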(event OnComponentBeginOverlap(Box)
  (params (OverlappedComponent :type Primitive%20Component%20Object%20Reference) (OtherActor :type Actor%20Object%20Reference) (OtherComp :type Primitive%20Component%20Object%20Reference) (OtherBodyIndex :type Integer) (bFromSweep :type Boolean) (SweepResult :type Hit%20Result%20Structure%20%28by%20ref%29))
  (bind _ascharacter (Utilities|Casting|CastToCharacter OtherActor)
    (:then
      (Character|LaunchCharacter _ascharacter "0.000000,0.000000,1000.000000" false false))
    (:CastFailed
      (if (Physics|IsSimulatingPhysics OtherComp "None")
        (Class|PrimitiveComponent|AddVelocityChangeImpulseatLocation OtherComp "0.000000,0.000000,2000.000000" (Transformation|GetWorldLocation OtherComp) "None")))))

(event EventBeginPlay
  (Utilities|FlowControl|Delay (Variables|Default|GetMainTornadoDuration))
  (Development|PrintString "Hello")
  (Components|Activation|Deactivate (Variables|Default|GetNS_TornadoEffect))
  (Collision|SetCollisionEnabled (Variables|Default|GetBox) "NoCollision")
  (Utilities|FlowControl|Delay 3.0)
  (Actor|DestroyActor))

(fn ConstructionScript)