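; Wind tornado spell that throws a wind ball from the player's left hand.
; DoSpell spawns BP_WindBallFX at the SpellLHand socket, aimed along the first-person camera, and plays the throw montage.
; The spell passes its tornado duration and push scale to the spawned ball; the tornado behavior itself is not in this Blueprint.
; Leftover nodes for attaching to a weapon socket are unwired.
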(event EventBeginPlay)

(fn ConstructionScript)

(fn DoSpell
  (params (Player :type BP%20Apex%20Character%20Object%20Reference))
  (Game|SpawnActorfromClass "/Game/_Project/BP/BP_FX/WindBall/BP_WindBallFX.BP_WindBallFX_C" (Math|Transform|MakeTransform (.Location (Math|Transform|BreakTransform (Transformation|GetSocketTransform (Variables|/Script/Engine.Character|GetMesh Player) "SpellLHand" "RTS_World"))) (Math|Conversions|RotationFromXVector (Math|Vector|GetForwardVector (Variables|/Game/_Project/BP/BP_ApexCharacter.BP_ApexCharacter_C|GetFirstPersonCamera Player)))) "AlwaysSpawn" "MultiplyWithRoot" (Variables|Default|GetWindBallFx) (Variables|Default|GetTornadoDuration) (Variables|Default|GetTornadoPushScale) 0)
  (Animation|PlayAnimMontage Player "/Game/_Project/Assets/Characters/Animations/Spells/Montages/AM_Spell_Throw.AM_Spell_Throw" 1.0 "None"))