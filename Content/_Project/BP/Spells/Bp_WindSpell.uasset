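; Wind spell actor that launches a wind ball effect from the player's left weapon socket when cast.
; DoSpell spawns BP_WindBallFX at that socket, aimed along the first-person camera's forward vector, and passes it the tornado duration.
; The spell actor then destroys itself, so it is single-use.
; Event graph logic is empty, and leftover socket-attachment nodes in DoSpell never run.
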(event EventBeginPlay)

(event Collision|EventActorBeginOverlap
  (params (OtherActor :type Actor%20Object%20Reference)))

(event EventTick
  (params (DeltaSeconds :type Float%20%28single-precision%29)))

(fn ConstructionScript)

(fn DoSpell
  (params (Player :type BP%20Apex%20Character%20Object%20Reference))
  (Game|SpawnActorfromClass "/Game/_Project/BP/BP_FX/WindBall/BP_WindBallFX.BP_WindBallFX_C" (Math|Transform|MakeTransform (.Location (Math|Transform|BreakTransform (Transformation|GetSocketTransform (Variables|/Script/Engine.Character|GetMesh Player) "weapon_lSocket" "RTS_World"))) (Math|Conversions|RotationFromXVector (Math|Vector|GetForwardVector (Variables|/Game/_Project/BP/BP_ApexCharacter.BP_ApexCharacter_C|GetFirstPersonCamera Player)))) "AlwaysSpawn" "MultiplyWithRoot" (Variables|Default|GetWindBallFx) (Variables|Default|GetTornadoDuration) 0)
  (Actor|DestroyActor))