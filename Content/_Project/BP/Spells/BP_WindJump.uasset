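; BP_WindJump is a spell that triggers on the player's jumps when the jump count exceeds one.
; Initialize stores the player and binds to the ParkourComponent's pre-normal-jump dispatcher, whose handler calls DoSpell for those repeat jumps.
; DoSpell runs the parent spell logic, then spawns BP_WindJumpFX at the player mesh's world transform.
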(event Custom|CE_DoJump
  (params (JumpCount :type Integer))
  (if (> JumpCount 1)
    (CallFunction|DoSpell (Variables|Default|GetPlayer))))

(event EventBeginPlay)

(event Collision|EventActorBeginOverlap
  (params (OtherActor :type Actor%20Object%20Reference)))

(event EventTick
  (params (DeltaSeconds :type Float%20%28single-precision%29)))

(fn ConstructionScript)

(fn DoSpell
  (params (Player :type BP%20Apex%20Character%20Object%20Reference))
  (|CallParentFunction Player)
  (Game|SpawnActorfromClass "/Game/_Project/BP/BP_FX/WindJump/BP_WindJumpFX.BP_WindJumpFX_C" (Transformation|GetWorldTransform (Variables|/Script/Engine.Character|GetMesh Player)) "Undefined" "MultiplyWithRoot" 0 0))

(fn Initialize
  (params (Player :type BP%20Apex%20Character%20Object%20Reference) (SpellInfo :type BPDA%20Spell%20Info%20Object%20Reference))
  (|CallParentFunction Player SpellInfo)
  (Variables|Default|SetPlayer Player)
  (EventDispatchers|BindEventtoEDPreNormalJump (Variables|/Game/_Project/BP/BP_ApexCharacter.BP_ApexCharacter_C|GetParkour%20Component Player) (EventDispatchers|CreateEvent :!event Custom|CE_DoJump)))