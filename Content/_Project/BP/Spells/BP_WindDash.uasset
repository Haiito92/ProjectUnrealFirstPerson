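; BP_WindDash is a dash spell that launches the player along the first-person camera's forward vector.
; DoSpell runs the parent logic, starts the cooldown, plays a casting sound and calls Launch on the player's ParkourComponent, scaled by the dash force.
; Its Niagara effect is created on the player on first cast, hidden from the owner, reactivated on later casts and deactivated after FXDuration rather than destroyed.
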(event Custom|DeactivateNiagara
  (bind _dashparticleeffect (Variables|Default|GetDashParticleEffect))
  (Utilities|FlowControl|Delay (Variables|Default|GetFXDuration))
  (Utilities|IsValid _dashparticleeffect
    (:Is%20Valid
      (Components|Activation|Deactivate _dashparticleeffect))))

(fn ConstructionScript)

(fn DoSpell
  (params (Player :type BP%20Apex%20Character%20Object%20Reference))
  (bind _dashparticleeffect (Variables|Default|GetDashParticleEffect))
  (|CallParentFunction Player)
  (CallFunction|CEStartCooldown)
  (Audio|PlaySound2D (Variables|Default|GetCastingSound) 1.0 1.0 0.0 0 0 false)
  (Utilities|IsValid _dashparticleeffect
    (:Is%20Valid
      (Components|Activation|Activate _dashparticleeffect true))
    (:Is%20Not%20Valid
      (|CreateNiagaraComponent Player)))
  (Default|Launch (Variables|/Game/_Project/BP/BP_ApexCharacter.BP_ApexCharacter_C|GetParkour%20Component Player) (* (Math|Vector|GetForwardVector (Variables|/Game/_Project/BP/BP_ApexCharacter.BP_ApexCharacter_C|GetFirstPersonCamera Player)) (Variables|Default|GetDashFirce)) false false false)
  (CallFunction|DeactivateNiagara))