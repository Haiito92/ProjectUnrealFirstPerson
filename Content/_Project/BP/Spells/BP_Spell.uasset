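; BP_Spell is a base spell Blueprint with overridable hooks for casting, stepping, resetting and adding or removing effects.
; Initialize stores a SpellInfo, whose cooldown and duration drive timers that clear the OnCooldown and Active flags, both exposed through getters.
; A separate timer event sets CanStep true after a given delay.
; The hooks are empty here, except Step, which prints a default debug message.
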(event Custom|CE_ReEnableStep
  (params (Delay :type Float%20%28single-precision%29))
  (Utilities|Time|SetTimerbyEvent (delegate Custom|StepEnable) Delay))

(event Custom|StepEnable
  (Variables|Default|SetCanStep true))

(event Custom|CE_ActivateSpell
  (Variables|Default|SetActive true)
  (Utilities|Time|SetTimerbyEvent (delegate Custom|DeactivateSpell) (Variables|/Game/_Project/Data/Blueprints/BPDA_SpellInfo.BPDA_SpellInfo_C|GetSpellDuration (Variables|Default|GetSpellInfo))))

(event Custom|DeactivateSpell
  (Variables|Default|SetActive false))

(event Custom|CE_StartCooldown
  (Variables|Default|SetOnCooldown true)
  (Utilities|Time|SetTimerbyEvent (delegate Custom|EnableSpell) (Variables|/Game/_Project/Data/Blueprints/BPDA_SpellInfo.BPDA_SpellInfo_C|GetSpellCooldown (Variables|Default|GetSpellInfo))))

(event Custom|EnableSpell
  (Variables|Default|SetOnCooldown false))

(fn ConstructionScript)

(fn DoSpell
  (params (Player :type BP%20Apex%20Character%20Object%20Reference)))

(fn Step
  (params (Player :type BP%20Apex%20Character%20Object%20Reference))
  (Development|PrintString "Default Stepp"))

(fn Reset
  (params (Player :type BP%20Apex%20Character%20Object%20Reference)))

(fn AddEffect
  (params (Player :type BP%20Apex%20Character%20Object%20Reference)))

(fn RemoveEffect
  (params (Player :type BP%20Apex%20Character%20Object%20Reference)))

(fn Initialize
  (params (Player :type BP%20Apex%20Character%20Object%20Reference) (SpellInfo :type BPDA%20Spell%20Info%20Object%20Reference))
  (Variables|Default|SetSpellInfo SpellInfo))

(fn IsonCooldown
  (return (Variables|Default|GetOnCooldown)))

(fn IsActive
  (return (Variables|Default|GetActive)))