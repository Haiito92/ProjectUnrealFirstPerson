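; BP_WindPlatform is an ultimate spell that spawns temporary wind platforms below the player and boosts parkour movement.
; Step, gated by remaining uses and a re-enable delay, calls DoSpell to spawn BP_WindPlatformFX, play the casting sound and decrement the count.
; Step only casts at four or fewer uses, while Reset restores five.
; AddEffect multiplies move speed and jump force, but RemoveEffect restores only move speed.
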(event EventBeginPlay)

(event Collision|EventActorBeginOverlap
  (params (OtherActor :type Actor%20Object%20Reference)))

(event EventTick
  (params (DeltaSeconds :type Float%20%28single-precision%29)))

(fn ConstructionScript)

(fn DoSpell
  (params (Player :type BP%20Apex%20Character%20Object%20Reference))
  (bind _returnvalue (Transformation|GetActorTransform Player))
  (Game|SpawnActorfromClass "/Game/_Project/BP/BP_FX/WindPlatform/BP_WindPlatformFX.BP_WindPlatformFX_C" (Math|Transform|MakeTransform (- (.location _returnvalue) "0.000000,0.000000,200.000000") (.rotation _returnvalue)) "Undefined" "MultiplyWithRoot" (Variables|Default|GetWindPlatformFX) (Variables|Default|GetWindPlatformDuration) 0)
  (Audio|PlaySound2D (Variables|Default|GetCastingSound) 1.0 1.0 0.0 0 0 false)
  (Math|Integer|DecrementInt (Variables|Default|GetNumberOfUltLeft)))

(fn Step
  (params (Player :type BP%20Apex%20Character%20Object%20Reference))
  (if (and (Variables|Default|GetCanStep) (> (Variables|Default|GetNumberOfUltLeft) 0))
    (if (<= (Variables|Default|GetNumberOfUltLeft) 4)
      (Variables|Default|SetCanStep false)
      (CallFunction|DoSpell Player)
      (CallFunction|CEReEnableStep 1.0))))

(fn Reset
  (params (Player :type BP%20Apex%20Character%20Object%20Reference))
  (Variables|Default|SetNumberOfUltLeft 5))

(fn AddEffect
  (params (Player :type BP%20Apex%20Character%20Object%20Reference))
  (bind _parkour_component (Variables|/Game/_Project/BP/BP_ApexCharacter.BP_ApexCharacter_C|GetParkour%20Component Player))
  (bind _speedultmultiplier (Variables|Default|GetSpeedUltMultiplier))
  (Default|SetMoveSpeedMultiplier _parkour_component _speedultmultiplier)
  (Default|SetGlobalJumpForceMultiplier _parkour_component _speedultmultiplier))

(fn RemoveEffect
  (params (Player :type BP%20Apex%20Character%20Object%20Reference))
  (Default|SetMoveSpeedMultiplier (Variables|/Game/_Project/BP/BP_ApexCharacter.BP_ApexCharacter_C|GetParkour%20Component Player) (Variables|/Game/_Project/Data/Blueprints/BPDA_CharacterInfo.BPDA_CharacterInfo_C|GetMoveSpeed (Variables|/Game/_Project/BP/BP_ApexCharacter.BP_ApexCharacter_C|GetCharacterInfo Player))))