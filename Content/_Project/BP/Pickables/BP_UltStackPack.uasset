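; BP_UltStackPack is a pickup that grants an ultimate stack to a BP_ApexCharacter.
; Sphere overlap calls AddUltStack on the character's SpellCastingComponent.
; When that call returns false, the pack calls ItemPickedUp and destroys itself.
; It also defines a DoHeal function for flat or max-HP percentage healing, which nothing in this Blueprint calls.
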(event OnComponentBeginOverlap(Sphere)
  (params (OverlappedComponent :type Primitive%20Component%20Object%20Reference) (OtherActor :type Actor%20Object%20Reference) (OtherComp :type Primitive%20Component%20Object%20Reference) (OtherBodyIndex :type Integer) (bFromSweep :type Boolean) (SweepResult :type Hit%20Result%20Structure%20%28by%20ref%29))
  (bind _asbp_apex_character (Utilities|Casting|CastToBP_ApexCharacter OtherActor))
  (bind _ismax (Default|AddUltStack (Variables|/Game/_Project/BP/BP_ApexCharacter.BP_ApexCharacter_C|GetSpellCastingComponent _asbp_apex_character)))
  (if (not _ismax)
    (Default|CallItemPickedUp)
    (Actor|DestroyActor)))

(event EventBeginPlay)

(event Collision|EventActorBeginOverlap
  (params (OtherActor :type Actor%20Object%20Reference)))

(event EventTick
  (params (DeltaSeconds :type Float%20%28single-precision%29)))

(fn ConstructionScript)

(fn DoHeal
  (params (Player :type BP%20Apex%20Character%20Object%20Reference))
  (bind _healed (Default|Heal Player (Math|Float|SelectFloat (* (Variables|Default|GetHealAmount) (Variables|/Game/_Project/Data/Blueprints/BPDA_CharacterInfo.BPDA_CharacterInfo_C|GetMaxHp (Variables|/Game/_Project/BP/BP_ApexCharacter.BP_ApexCharacter_C|GetCharacterInfo Player))) (Variables|Default|GetHealAmount) (Variables|Default|GetHealIsPercentHP))))
  (return _healed))