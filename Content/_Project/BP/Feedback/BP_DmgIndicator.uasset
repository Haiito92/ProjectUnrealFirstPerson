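; BP_DmgIndicator is a short-lived actor that shows a floating damage number near a hit target through a widget.
; On BeginPlay it treats its Owner as the damage dealer, passes Damage to the widget and scales itself by dealer-to-target distance, within clamped limits.
; A timeline lerps it between randomized, scale-adjusted offsets up and along the dealer's right vector, turning it toward the dealer, then destroys it.
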(event EventBeginPlay
  (Variables|Default|SetDmgDealer (Components|GetOwner))
  (Class|INDamageIndicator|PassDmg(Message) (UserInterface|GetWidget (Variables|Default|GetWidget)) (Variables|Default|GetDamage))
  (CallFunction|CalculateScale)
  (bind _location (CallFunction|GetStartLocation))
  (bind _location_2 (CallFunction|GetEndLocation))
  (bind _alpha (Timeline|MoveDmgIndicator PlayFromStart)
    (:Update
      (Transformation|SetActorLocationAndRotation (Math|Vector|Lerp(Vector) _location _location_2 _alpha) (Math|Rotator|FindLookatRotation (Transformation|GetActorLocation) (Transformation|GetActorLocation (Variables|Default|GetDmgDealer)))))
    (:Finished
      (Actor|DestroyActor))))

(fn ConstructionScript)

(fn GetEndLocation
  (bind _taget (Variables|Default|GetTaget))
  (return (+ (+ (* (Math|Random|RandomFloatinRange 6e+01 1e+02) (Transformation|GetActorUpVector _taget) (Variables|Default|GetScale)) (* (Math|Random|RandomFloatinRange 6e+01 1e+02) (Transformation|GetActorRightVector (Variables|Default|GetDmgDealer)) (Variables|Default|GetScale))) (Transformation|GetActorLocation _taget))))

(fn GetStartLocation
  (bind _taget (Variables|Default|GetTaget))
  (return (+ (+ (* (Math|Random|RandomFloatinRange 1e+01 2e+01) (Transformation|GetActorUpVector _taget) (Variables|Default|GetScale)) (* (Math|Random|RandomFloatinRange 1e+01 2e+01) (Transformation|GetActorRightVector (Variables|Default|GetDmgDealer)) (Variables|Default|GetScale))) (Transformation|GetActorLocation _taget))))

(fn CalculateScale
  (bind _output_get (Variables|Default|SetScale (Math|Float|Clamp(Float) (/ (* (/ (Math|Vector|VectorLength (- (Transformation|GetActorLocation (Variables|Default|GetDmgDealer)) (Transformation|GetActorLocation (Variables|Default|GetTaget)))) 1e+02) (Variables|Default|GetDistanceMultiplier)) (Variables|Default|GetBaseScaleDistance)) 1.0 7.0)))
  (Transformation|SetActorScale3D (Math|Conversions|ToVector(Float) _output_get)))