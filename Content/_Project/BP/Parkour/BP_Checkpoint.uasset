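; BP_Checkpoint is a parkour checkpoint trigger that updates an overlapping actor's checkpoint and can control its timer.
; On box overlap, it passes the ForwardArrow's location, raised slightly, and rotation to the actor's BP_ParkourModeComponent.
; Boolean flags then start, stop or reset that component's timer, in that priority order.
; The construction script sizes the box from BoxExtent, and BeginPlay destroys the Rubik component.
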(event OnComponentBeginOverlap(Box)
  (params (OverlappedComponent :type Primitive%20Component%20Object%20Reference) (OtherActor :type Actor%20Object%20Reference) (OtherComp :type Primitive%20Component%20Object%20Reference) (OtherBodyIndex :type Integer) (bFromSweep :type Boolean) (SweepResult :type Hit%20Result%20Structure%20%28by%20ref%29))
  (bind _returnvalue (Actor|GetComponentbyClass OtherActor "/Game/_Project/BP/Components/BP_ParkourModeComponent.BP_ParkourModeComponent_C"))
  (bind _forwardarrow (Variables|Default|GetForwardArrow))
  (bind _returnvalue_2 (Transformation|GetWorldTransform _forwardarrow))
  (Utilities|IsValid _returnvalue
    (:Is%20Valid
      (Default|CheckpointUpdate _returnvalue (Math|Transform|MakeTransform (+ (.location _returnvalue_2) "0.000000,0.000000,96.000000") (.rotation _returnvalue_2) "1.000000,1.000000,1.000000"))
      (if (Variables|Default|GetStartTimer)
        (Default|StartTimer _returnvalue)
        (elif (Variables|Default|GetStopTimer)
          (Default|StopTimer _returnvalue)
          (elif (Variables|Default|GetResetTimer)
            (Default|ResetTimer _returnvalue)))))))

(event EventBeginPlay
  (Components|DestroyComponent (Variables|Default|GetRubik)))

(event Collision|EventActorBeginOverlap
  (params (OtherActor :type Actor%20Object%20Reference)))

(event EventTick
  (params (DeltaSeconds :type Float%20%28single-precision%29)))

(fn ConstructionScript
  (Components|Box|SetBoxExtent (Variables|Default|GetBox) (Variables|Default|GetBox%20Extent) true))