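; BP_ParkourEndZone is the exit trigger volume for the parkour mode, tracking players who stand inside its box.
; Entering or leaving sets the waiting state on the actor's BP_ParkourModeComponent and adds or removes an exiting player on BP_ParkourGameMode.
; When AddExitingPlayer returns true, it loads MenusLevel and removes the second local player controller if one exists.
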(event OnComponentBeginOverlap(Box)
  (params (OverlappedComponent :type Primitive%20Component%20Object%20Reference) (OtherActor :type Actor%20Object%20Reference) (OtherComp :type Primitive%20Component%20Object%20Reference) (OtherBodyIndex :type Integer) (bFromSweep :type Boolean) (SweepResult :type Hit%20Result%20Structure%20%28by%20ref%29))
  (bind _returnvalue (Actor|GetComponentbyClass OtherActor "/Game/_Project/BP/Components/BP_ParkourModeComponent.BP_ParkourModeComponent_C"))
  (bind _returnvalue_2 (Game|GetPlayerController 1))
  (Utilities|FlowControl|Sequence
    (:then_0
      (Utilities|IsValid _returnvalue
        (:Is%20Valid
          (Default|CESetWaitingState _returnvalue true))))
    (:then_1
      (if (Utilities|DoesObjectImplementInterface OtherActor "/Game/_Project/Interfaces/IN_Player.IN_Player_C")
        (bind _allplayersleaving (Default|AddExitingPlayer (Variables|Default|GetGameMode)))
        (if _allplayersleaving
          (Game|OpenLevel(byName) "MenusLevel")
          (Utilities|IsValid _returnvalue_2
            (:Is%20Valid
              (Class|GameplayStatics|RemovePlayer _returnvalue_2 false))))))))

(event OnComponentEndOverlap(Box)
  (params (OverlappedComponent :type Primitive%20Component%20Object%20Reference) (OtherActor :type Actor%20Object%20Reference) (OtherComp :type Primitive%20Component%20Object%20Reference) (OtherBodyIndex :type Integer))
  (bind _returnvalue (Actor|GetComponentbyClass OtherActor "/Game/_Project/BP/Components/BP_ParkourModeComponent.BP_ParkourModeComponent_C"))
  (Utilities|FlowControl|Sequence
    (:then_0
      (Utilities|IsValid _returnvalue
        (:Is%20Valid
          (Default|CESetWaitingState _returnvalue false))))
    (:then_1
      (if (Utilities|DoesObjectImplementInterface OtherActor "/Game/_Project/Interfaces/IN_Player.IN_Player_C")
        (Default|RemoveExitingPlayer (Variables|Default|GetGameMode))))))

(event EventBeginPlay
  (bind _asbp_parkour_game_mode (Utilities|Casting|CastToBP_ParkourGameMode (Game|GetGameMode)))
  (Variables|Default|SetGameMode _asbp_parkour_game_mode))

(event Collision|EventActorBeginOverlap
  (params (OtherActor :type Actor%20Object%20Reference)))

(event EventTick
  (params (DeltaSeconds :type Float%20%28single-precision%29)))

(fn ConstructionScript)