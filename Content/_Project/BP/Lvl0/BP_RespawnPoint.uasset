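; A respawn point actor that reports itself as disabled while any player character stands inside its detection capsule.
; Capsule begin and end overlaps adjust a count of BP_ApexCharacter occupants, and IsDisabled returns true while that count is above zero.
; The construction script sizes the capsule from Radius and HalfHeight, caps radius at half-height, and raises it by half that half-height.
; The PlayerPrev component is destroyed on BeginPlay.
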(event OnComponentBeginOverlap(PlayerDetection)
  (params (OverlappedComponent :type Primitive%20Component%20Object%20Reference) (OtherActor :type Actor%20Object%20Reference) (OtherComp :type Primitive%20Component%20Object%20Reference) (OtherBodyIndex :type Integer) (bFromSweep :type Boolean) (SweepResult :type Hit%20Result%20Structure%20%28by%20ref%29))
  (Utilities|Casting|CastToBP_ApexCharacter OtherActor)
  (Math|Integer|IncrementInt (Variables|Default|GetOverlappedPlayersCount)))

(event OnComponentEndOverlap(PlayerDetection)
  (params (OverlappedComponent :type Primitive%20Component%20Object%20Reference) (OtherActor :type Actor%20Object%20Reference) (OtherComp :type Primitive%20Component%20Object%20Reference) (OtherBodyIndex :type Integer))
  (Utilities|Casting|CastToBP_ApexCharacter OtherActor)
  (Math|Integer|DecrementInt (Variables|Default|GetOverlappedPlayersCount)))

(event EventBeginPlay
  (Components|DestroyComponent (Variables|Default|GetPlayerPrev)))

(event Collision|EventActorBeginOverlap
  (params (OtherActor :type Actor%20Object%20Reference)))

(event EventTick
  (params (DeltaSeconds :type Float%20%28single-precision%29)))

(fn ConstructionScript
  (bind _playerdetection (Variables|Default|GetPlayerDetection))
  (Components|Capsule|SetCapsuleSize _playerdetection (Math|Float|Min(Float) (Variables|Default|GetRadius) (Variables|Default|GetHalfHeight)) (Variables|Default|GetHalfHeight) true)
  (Transformation|SetRelativeLocation _playerdetection (Math|Vector|MakeVector 0.0 0.0 (/ (Variables|Default|GetHalfHeight) 2.0)) false false))

(fn IsDisabled
  (return (> (Variables|Default|GetOverlappedPlayersCount) 0)))