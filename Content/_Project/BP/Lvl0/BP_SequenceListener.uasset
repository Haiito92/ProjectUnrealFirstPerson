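; Level sequence listener actor that starts the music and hands control to the game mode when the sequence ends or is skipped.
; On BeginPlay it caches BP_ApexGameModeBase, triggers its music and grabs a LevelSequenceActor from the level.
; A skip event stops the player at the current time and runs the end event.
; The end event calls the game mode's begin event and fires SequenceEnd.
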(event Custom|CE_OnSequenceEnd
  (Default|CEBegin (Variables|Default|GetGameMode))
  (Default|CallSequenceEnd))

(event Custom|CE_Skip
  (bind _levelsequence (Variables|Default|GetLevelSequence))
  (bind _sequenceplayer (Variables|/Script/LevelSequence.LevelSequenceActor|GetSequencePlayer _levelsequence))
  (Utilities|IsValid _sequenceplayer
    (:Is%20Valid
      (Class|MovieSceneSequencePlayer|StopatCurrentTime _sequenceplayer)
      (CallFunction|CEonSequenceEnd))))

(event EventBeginPlay
  (bind _asapex_gamemode_base (Utilities|Casting|CastToBP_ApexGameModeBase (Game|GetGameMode)))
  (bind _output_get (Variables|Default|SetGameMode _asapex_gamemode_base))
  (Default|CEStartMusic _output_get)
  (bind _returnvalue (Actor|GetActorOfClass "/Script/LevelSequence.LevelSequenceActor"))
  (Variables|Default|SetLevelSequence _returnvalue))

(event Collision|EventActorBeginOverlap
  (params (OtherActor :type Actor%20Object%20Reference)))

(event EventTick
  (params (DeltaSeconds :type Float%20%28single-precision%29)))

(fn ConstructionScript)