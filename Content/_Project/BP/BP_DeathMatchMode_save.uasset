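; Deathmatch game mode for local multiplayer that creates and possesses a player character at each PlayerStart.
; Combat events update a per-player score map of kills, damage, shots, hits and headshots.
; Deaths lead to a delayed respawn at a random point, retrying disabled ones up to a capped count.
; Depending on game instance settings, a kill target or looping timer ends the match, triggering time dilation through a spawned BP_TimeDilator.
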(event Custom|CE_DoTimer
  ;[1 1 1] Increment Timer and check if over
  (if (not (Variables|Default|GetIsOver))
    (bind _result (Math|Integer|IncrementInt (Variables|Default|GetTimer))
      (:%20%20
        (if (>= _result (.timeramount (Variables|/Game/_Project/BP/BP_ApexGameInstance.BP_ApexGameInstance_C|GetGamemodeInfo (Variables|Default|GetGameInstance))))
          (bind _playerindex (CallFunction|FindPlayerwithMostKills))
          (CallFunction|CEEndGame _playerindex))))))

(event Custom|CE_BulletHit
  (params (PlayerIndex :type Integer) (IsHeadShot :type Boolean))
  (bind _playerscores (Variables|Default|GetPlayerScores))
  (bind _value (Utilities|Map|Find _playerscores PlayerIndex))
  (bind (_bulletshit _headshothits) (Utilities|Struct|BreakST_PlayerScore _value))
  ;[1 1 1] Player Hit another Player with a bullet
  (if (not (Variables|Default|GetIsOver))
    (bind _structout (Utilities|Struct|SetmembersinST_PlayerScore _value (+ _bulletshit 1) (+ _headshothits (Math|Integer|SelectInt 1 0 IsHeadShot))))
    (Utilities|Map|Add (Variables|Default|GetPlayerScores) PlayerIndex _structout)))

(event Custom|CE_PlayerDeath
  (params (Killer :type BP%20Apex%20Character%20Object%20Reference) (PlayerDead :type BP%20Apex%20Character%20Object%20Reference))
  ;[1 1 1] Logic called when a Player is killed
  (if (not (Variables|Default|GetIsOver))
    (|UpdateScores Killer PlayerDead
      (:execute
        (Default|CallPlayerDeath Killer PlayerDead)
        (Default|Kill PlayerDead)
        (if (Utilities|Enum|NotEqual(Enum) (Utilities|GetGamemodeMode) "NewEnumerator1")
          (bind (_state _winnerplayerindex) (CallFunction|IsGameOverKills))
          (if _state
            (CallFunction|CEEndGame _winnerplayerindex)
            (else
              (Utilities|FlowControl|Delay (Variables|Default|GetTimeBeforeRespawn) :!label _label)
              (Widget|RemovefromParent (Variables|/Game/_Project/BP/BP_ApexCharacter.BP_ApexCharacter_C|GetGUI PlayerDead))
              (CallFunction|RespawnPlayer (Variables|/Game/_Project/BP/BP_ApexCharacter.BP_ApexCharacter_C|GetPlayerIndex PlayerDead) (Variables|/Game/_Project/BP/BP_ApexCharacter.BP_ApexCharacter_C|GetCharacterInfo PlayerDead))
              (Actor|DestroyActor PlayerDead)))
          (else
            (goto _label)))))))

(event Custom|CE_BulletShot
  (params (PlayerIndex :type Integer))
  (bind _playerscores (Variables|Default|GetPlayerScores))
  (bind _value (Utilities|Map|Find _playerscores PlayerIndex))
  ;[1 1 1] Player Fired a bullet
  (if (not (Variables|Default|GetIsOver))
    (bind _structout (Utilities|Struct|SetmembersinST_PlayerScore _value (+ (Utilities|Struct|BreakST_PlayerScore _value) 1)))
    (Utilities|Map|Add (Variables|Default|GetPlayerScores) PlayerIndex _structout)))

(event Custom|CE_AddDamageScore
  (params (DmgDealer :type BP%20Apex%20Character%20Object%20Reference) (DmgAmount :type Float%20%28double-precision%29))
  (bind _playerscores (Variables|Default|GetPlayerScores))
  (bind _playerindex (Variables|/Game/_Project/BP/BP_ApexCharacter.BP_ApexCharacter_C|GetPlayerIndex DmgDealer))
  (bind _value (Utilities|Map|Find _playerscores _playerindex))
  ;[1 1 1] Add Damage dealt by Player to his score
  (if (not (Variables|Default|GetIsOver))
    (bind _structout (Utilities|Struct|SetmembersinST_PlayerScore _value (+ (Utilities|Struct|BreakST_PlayerScore _value) DmgAmount)))
    (Utilities|Map|Add (Variables|Default|GetPlayerScores) (Variables|/Game/_Project/BP/BP_ApexCharacter.BP_ApexCharacter_C|GetPlayerIndex DmgDealer) _structout)))

(event Custom|CE_EndGame
  (params (WinnerPlayerIndex :type Integer))
  (if (not (Variables|Default|GetIsOver))
    (Development|PrintString (Utilities|String|BuildString(Integer) "" "Player " WinnerPlayerIndex " Won"))
    (Variables|Default|SetIsOver true)
    (Default|CEEndGameTimeDilation (Variables|Default|GetTimeDilator))))

(event EventBeginPlay
  (CallFunction|SpawnPlayers)
  (bind _outactors (Actor|GetAllActorsOfClass "/Game/_Project/BP/Lvl0/BP_RespawnPoint.BP_RespawnPoint_C"))
  (for _array_element _outactors
    (Utilities|Array|Add (Variables|Default|GetRespawnPoints) _array_element))
  (bind _asbp_apex_game_instance (Utilities|Casting|CastToBP_ApexGameInstance (Game|GetGameInstance)))
  (Variables|Default|SetGameInstance _asbp_apex_game_instance)
  (Utilities|FlowControl|Sequence
    (:then_0
      (if (Utilities|Enum|NotEqual(Enum) (Utilities|GetGamemodeMode) "NewEnumerator0")
        (Utilities|Time|SetTimerbyEvent (EventDispatchers|CreateEvent :!event Custom|CE_DoTimer) 1.0 true)))
    (:then_1
      (bind _returnvalue (Game|SpawnActorfromClass "/Game/_Project/BP/Lvl0/BP_TimeDilator.BP_TimeDilator_C" (Math|Transform|MakeTransform "0, 0, 0" "0, 0, 0" "1.000000,1.000000,1.000000") "Undefined" "MultiplyWithRoot" 0 0))
      (Variables|Default|SetTimeDilator _returnvalue))))

(fn ConstructionScript)

(fn SpawnPlayers
  (bind _outactors (Actor|GetAllActorsOfClass "/Script/Engine.PlayerStart"))
  (for (_array_element _array_index) _outactors
    (bind _output_get (Variables|Default|SetArray%20Index _array_index))
    (bind _returnvalue (Class|GameplayStatics|CreatePlayer _output_get)) ; Create local player controller
    (Input|AddMappingContext (PlayerController|LocalPlayerSubsystems|GetEnhancedInputLocalPlayerSubsystem (select (== (Variables|Default|GetArray%20Index) 0) (Game|GetPlayerController 0) _returnvalue)) "/Game/_Project/Input/IMC_Default.IMC_Default" 0 "(bIgnoreAllPressedKeysUntilRelease=True,bForceImmediately=False,bNotifyUserSettings=False)") ; Assign the input mapping to the player
    (bind _returnvalue_2 (Game|SpawnActorfromClass "/Game/_Project/BP/BP_ApexCharacter.BP_ApexCharacter_C" (Transformation|GetActorTransform _array_element) "Undefined" "MultiplyWithRoot" 0 "/Game/_Project/Data/DA_TEstCharacter.DA_TEstCharacter" (Variables|Default|GetArray%20Index) 0))
    (Pawn|Possess (Game|GetPlayerController (Variables|Default|GetArray%20Index)) _returnvalue_2) ; Assign controller to player
    (Utilities|Map|Add (Variables|Default|GetPlayerScores) (|Copy (Variables|Default|GetArray%20Index)) (|Copy (Utilities|Struct|MakeST_PlayerScore)))))

(fn RespawnPlayer
  (params (Player%20Index :type Integer) (CharacterInfo :type BPDA%20Character%20Info%20Object%20Reference))
  (bind _returnvalue (Game|GetPlayerController Player%20Index))
  (bind _output_get (LocalVariables|SetSpawnPoint (.OutItem (Utilities|Array|Random (Variables|Default|GetRespawnPoints)))))
  (while (and (Default|IsDisabled _output_get) (< (LocalVariables|GetLoopIterations) 50))
    ;[1 1 1] Try to get a spawn point that is not disabled, else go brrr
    (LocalVariables|SetSpawnPoint (.OutItem (Utilities|Array|Random (Variables|Default|GetRespawnPoints))))
    (Math|Integer|IncrementInt (LocalVariables|GetLoopIterations)))
  (bind _returnvalue_2 (Game|SpawnActorfromClass "/Game/_Project/BP/BP_ApexCharacter.BP_ApexCharacter_C" (Math|Transform|MakeTransform (+ (.location (Transformation|GetActorTransform (LocalVariables|GetSpawnPoint))) "0.000000,0.000000,96.000000") (.rotation (Transformation|GetActorTransform (LocalVariables|GetSpawnPoint))) (.scale (Transformation|GetActorTransform (LocalVariables|GetSpawnPoint)))) "AlwaysSpawn" "MultiplyWithRoot" 0 CharacterInfo Player%20Index 0))
  (Pawn|Possess _returnvalue _returnvalue_2) ; Assign controller to player
  (Default|CallPlayerRespawn _returnvalue_2)
  (bind _asbp_apex_player_controller (Utilities|Casting|CastToBP_ApexPlayerController _returnvalue))
  (Default|OnPlayerRespawn _asbp_apex_player_controller))

(fn IsGameOverKills
  (bind _values (Utilities|Map|Values (Variables|Default|GetPlayerScores)))
  (for (_array_element _array_index) _values
    (if (>= (Utilities|Struct|BreakST_PlayerScore _array_element) (.requiredkillsamount (Variables|/Game/_Project/BP/BP_ApexGameInstance.BP_ApexGameInstance_C|GetGamemodeInfo (Variables|Default|GetGameInstance))))
      (return true _array_index)))
  (return false 0))

(fn FindPlayerwithMostKills
  (bind _values (Utilities|Map|Values (Variables|Default|GetPlayerScores)))
  (for (_array_element _array_index) _values
    (if (> (Utilities|Struct|BreakST_PlayerScore _array_element) (LocalVariables|GetLastKillNumber))
      (LocalVariables|SetLastKillNumber (Utilities|Struct|BreakST_PlayerScore _array_element))
      (LocalVariables|SetPlayerID _array_index)))
  (return (LocalVariables|GetPlayerID)))