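; BP_CamDirector drives the main menu camera, gliding one moving camera actor between look-at points mapped to each menu.
; On BeginPlay it waits a tick, gets the menu widget from the HUD, binds to its menu-changed callback and sets the camera as view target.
; It snaps to the game instance's starting menu.
; MoveCamToPos looks up the menu's actor and moves the camera's scene component to that transform over the given time.
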(event Custom|MoveCamToPos
  (params (Menu :type EMenus%20Enum :default "NewEnumerator4") (Time :type Float%20%28double-precision%29))
  (bind _maplookats (Variables|Default|GetMapLookAts))
  (bind (_value _returnvalue) (Utilities|Map|Find _maplookats Menu))
  (bind _returnvalue_2 (Transformation|GetActorTransform _value))
  ;[0.05098 0.05098 0.05098] MoveCam
  (if _returnvalue
    (Components|MoveComponentTo (Variables|/Script/Engine.CameraActor|GetSceneComponent (Variables|Default|GetMovingCamActor)) (.location _returnvalue_2) (.rotation _returnvalue_2) false false Time true)))

(event EventBeginPlay
  (Utilities|FlowControl|DelayUntilNextTick)
  ;[0.05098 0.05098 0.05098] GetMainMenu Widget
  (bind _aswd_main_menu_hud (Utilities|Casting|CastToWD_MainMenuHUD (HUD|GetHUD (Game|GetPlayerController 0))))
  (bind _mainmenu (Variables|/Game/_Project/Widgets/WD_MainMenuHUD.WD_MainMenuHUD_C|GetMainMenu _aswd_main_menu_hud)
    (:then
      (bind _output_get (Variables|Default|SetMainMenuWidget _mainmenu))
      ;[0.05098 0.05098 0.05098] Bind to Main Menu Callbacks
      (EventDispatchers|BindEventtoMenuChanged _output_get (EventDispatchers|CreateEvent :!event Custom|MoveCamToPos))
      (Game|Player|SetViewTargetwithBlend (Game|GetPlayerController 0) (Variables|Default|GetMovingCamActor) 0.0 "VTBlend_Linear" 0.0 false)
      (bind _asbp_apex_game_instance (Utilities|Casting|CastToBP_ApexGameInstance (Game|GetGameInstance)))
      (CallFunction|MoveCamtoPos (Variables|/Game/_Project/BP/BP_ApexGameInstance.BP_ApexGameInstance_C|GetMenuToStartFrom _asbp_apex_game_instance) 0.0))
    (:else)))

(fn ConstructionScript)