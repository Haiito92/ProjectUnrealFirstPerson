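; Spell-casting component that spawns and initializes a player's two spells, ultimate and passive as actors from CharacterInfo.
; Gates and flags separate single-trigger casts, which respect cooldowns, from a both-trigger ultimate press, also available through IA_Ult.
; The ultimate steps if already active, otherwise requires and consumes a full stack.
; Dispatchers broadcast casts and stack changes; the timer setup for disabling the ultimate is unconnected.
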(event Custom|CE_OnLeftTrigger
  (params (State :type EInputState%20Enum :default "NewEnumerator0"))
  (bind _player (Variables|Default|GetPlayer))
  (bind _character_info (Variables|Default|GetCharacter%20Info))
  (bind _spell1 (Variables|/Game/_Project/Data/Blueprints/BPDA_CharacterInfo.BPDA_CharacterInfo_C|GetSpell1 _character_info))
  (switch Utilities|FlowControl|Switch|SwitchonEInputState State
    (:NewEnumerator0
      (Utilities|FlowControl|Gate true :!label _label
        (:Exit
          (Variables|Default|SetTriggerL false :!label _label_2)
          (CallFunction|CECloseTriggerGates)
          (Utilities|FlowControl|Sequence
            (:then_0
              (Development|PrintString "Cast Spell"))
            (:then_1
              (if (Default|IsonCooldown (Variables|Default|GetSpell1))
                (Audio|PlaySound2D (Variables|Default|GetNoSpellSound) 1.0 1.0 0.0 0 0)
                (else
                  (Default|DoSpell (Variables|Default|GetSpell1) _player)
                  (Default|CallWhenASpellIsCast (Variables|/Game/_Project/Data/Blueprints/BPDA_SpellInfo.BPDA_SpellInfo_C|GetSpellCooldown _spell1) (Variables|/Game/_Project/Data/Blueprints/BPDA_SpellInfo.BPDA_SpellInfo_C|GetSpellType _spell1)))))))))
    (:NewEnumerator1
      (Utilities|FlowControl|Sequence
        (:then_0
          (goto _label Open))
        (:then_1
          (Variables|Default|SetTriggerL true)
          (if (Variables|Default|GetTriggerR)
            (Utilities|ResetTriggerInput)
            (CallFunction|CECloseTriggerGates)
            (Utilities|FlowControl|Sequence
              (:then_0
                (Development|PrintString "Cast Ult"))
              (:then_1
                (if (Default|IsActive (Variables|Default|GetUlt))
                  (Default|Step (Variables|Default|GetUlt) _player)
                  (elif (>= (Variables|Default|GetUltStack) (Variables|Default|GetUltStackMax))
                    (Utilities|CastUlt)
                    (else
                      (Audio|PlaySound2D (Variables|Default|GetNoSpellSound) 1.0 1.0 0.0 0 0))))))))))
    (:NewEnumerator2
      (if (Variables|Default|GetTriggerL)
        (goto _label_2)))))

(event Custom|CE_OnRightTrigger
  (params (State :type EInputState%20Enum :default "NewEnumerator0"))
  (bind _player (Variables|Default|GetPlayer))
  (bind _character_info (Variables|Default|GetCharacter%20Info))
  (bind _spell2 (Variables|/Game/_Project/Data/Blueprints/BPDA_CharacterInfo.BPDA_CharacterInfo_C|GetSpell2 _character_info))
  (switch Utilities|FlowControl|Switch|SwitchonEInputState State
    (:NewEnumerator0
      (Utilities|FlowControl|Gate true :!label _label
        (:Exit
          (Variables|Default|SetTriggerR false :!label _label_2)
          (CallFunction|CECloseTriggerGates)
          (Utilities|FlowControl|Sequence
            (:then_0
              (Development|PrintString "Cast Spell"))
            (:then_1
              (if (Default|IsonCooldown (Variables|Default|GetSpell2))
                (Audio|PlaySound2D (Variables|Default|GetNoSpellSound) 1.0 1.0 0.0 0 0)
                (else
                  (Default|DoSpell (Variables|Default|GetSpell2) _player)
                  (Default|CallWhenASpellIsCast (Variables|/Game/_Project/Data/Blueprints/BPDA_SpellInfo.BPDA_SpellInfo_C|GetSpellCooldown _spell2) (Variables|/Game/_Project/Data/Blueprints/BPDA_SpellInfo.BPDA_SpellInfo_C|GetSpellType _spell2)))))))))
    (:NewEnumerator1
      (Utilities|FlowControl|Sequence
        (:then_0
          (goto _label Open))
        (:then_1
          (Variables|Default|SetTriggerR true)
          (if (Variables|Default|GetTriggerL)
            (Utilities|ResetTriggerInput)
            (CallFunction|CECloseTriggerGates)
            (Utilities|FlowControl|Sequence
              (:then_0
                (Development|PrintString "Cast Ult"))
              (:then_1
                (if (Default|IsActive (Variables|Default|GetUlt))
                  (Default|Step (Variables|Default|GetUlt) _player)
                  (elif (>= (Variables|Default|GetUltStack) (Variables|Default|GetUltStackMax))
                    (Utilities|CastUlt)
                    (else
                      (Audio|PlaySound2D (Variables|Default|GetNoSpellSound) 1.0 1.0 0.0 0 0))))))))))
    (:NewEnumerator2
      (if (Variables|Default|GetTriggerR)
        (goto _label_2)))))

(event Custom|CE_DisableUlt
  (Development|PrintString "ULT FINISHED" true true "(R=1.000000,G=0.010213,B=0.000000,A=1.000000)")
  (Default|RemoveEffect (Variables|Default|GetUlt) (Variables|Default|GetPlayer))
  (Variables|Default|SetIsUltActive false))

(event Custom|CE_CloseTriggerGates
  (bind _character_info (Variables|Default|GetCharacter%20Info))
  (bind _character_info_2 (Variables|Default|GetCharacter%20Info))
  (bind _spell1 (Variables|/Game/_Project/Data/Blueprints/BPDA_CharacterInfo.BPDA_CharacterInfo_C|GetSpell1 _character_info))
  (bind _spell2 (Variables|/Game/_Project/Data/Blueprints/BPDA_CharacterInfo.BPDA_CharacterInfo_C|GetSpell2 _character_info_2))
  (Utilities|FlowControl|Sequence
    (:then_0
      (if (not (Variables|Default|GetTriggerL))
        (Utilities|FlowControl|Gate true) ; enters at Close
      ))
    (:then_1
      (if (not (Variables|Default|GetTriggerR))
        (Utilities|FlowControl|Gate true) ; enters at Close
      ))))

(event Custom|CE_Initialize
  (params (Player :type BP%20Apex%20Character%20Object%20Reference))
  (Variables|Default|SetPlayer Player)
  (Variables|Default|SetCharacter%20Info (Variables|/Game/_Project/BP/BP_ApexCharacter.BP_ApexCharacter_C|GetCharacterInfo (Variables|Default|GetPlayer)))
  (bind _outputspell (CallFunction|CreateSpell (Variables|/Game/_Project/Data/Blueprints/BPDA_SpellInfo.BPDA_SpellInfo_C|GetSpell (Variables|/Game/_Project/Data/Blueprints/BPDA_CharacterInfo.BPDA_CharacterInfo_C|GetSpell1 (Variables|/Game/_Project/BP/BP_ApexCharacter.BP_ApexCharacter_C|GetCharacterInfo (Variables|Default|GetPlayer))))))
  (bind _output_get (Variables|Default|SetSpell1 _outputspell))
  (Default|Initialize _output_get (Variables|Default|GetPlayer) (Variables|/Game/_Project/Data/Blueprints/BPDA_CharacterInfo.BPDA_CharacterInfo_C|GetSpell1 (Variables|/Game/_Project/BP/BP_ApexCharacter.BP_ApexCharacter_C|GetCharacterInfo (Variables|Default|GetPlayer))))
  (bind _outputspell_2 (CallFunction|CreateSpell (Variables|/Game/_Project/Data/Blueprints/BPDA_SpellInfo.BPDA_SpellInfo_C|GetSpell (Variables|/Game/_Project/Data/Blueprints/BPDA_CharacterInfo.BPDA_CharacterInfo_C|GetSpell2 (Variables|/Game/_Project/BP/BP_ApexCharacter.BP_ApexCharacter_C|GetCharacterInfo (Variables|Default|GetPlayer))))))
  (bind _output_get_2 (Variables|Default|SetSpell2 _outputspell_2))
  (Default|Initialize _output_get_2 (Variables|Default|GetPlayer) (Variables|/Game/_Project/Data/Blueprints/BPDA_CharacterInfo.BPDA_CharacterInfo_C|GetSpell2 (Variables|/Game/_Project/BP/BP_ApexCharacter.BP_ApexCharacter_C|GetCharacterInfo (Variables|Default|GetPlayer))))
  (bind _outputspell_3 (CallFunction|CreateSpell (Variables|/Game/_Project/Data/Blueprints/BPDA_SpellInfo.BPDA_SpellInfo_C|GetSpell (Variables|/Game/_Project/Data/Blueprints/BPDA_CharacterInfo.BPDA_CharacterInfo_C|GetSpellUlt (Variables|/Game/_Project/BP/BP_ApexCharacter.BP_ApexCharacter_C|GetCharacterInfo (Variables|Default|GetPlayer))))))
  (bind _output_get_3 (Variables|Default|SetUlt _outputspell_3))
  (Default|Initialize _output_get_3 (Variables|Default|GetPlayer) (Variables|/Game/_Project/Data/Blueprints/BPDA_CharacterInfo.BPDA_CharacterInfo_C|GetSpellUlt (Variables|/Game/_Project/BP/BP_ApexCharacter.BP_ApexCharacter_C|GetCharacterInfo (Variables|Default|GetPlayer))))
  (bind _outputspell_4 (CallFunction|CreateSpell (Variables|/Game/_Project/Data/Blueprints/BPDA_SpellInfo.BPDA_SpellInfo_C|GetSpell (Variables|/Game/_Project/Data/Blueprints/BPDA_CharacterInfo.BPDA_CharacterInfo_C|GetSpellPassive (Variables|/Game/_Project/BP/BP_ApexCharacter.BP_ApexCharacter_C|GetCharacterInfo (Variables|Default|GetPlayer))))))
  (bind _output_get_4 (Variables|Default|SetPassive _outputspell_4))
  (Default|Initialize _output_get_4 (Variables|Default|GetPlayer) (Variables|/Game/_Project/Data/Blueprints/BPDA_CharacterInfo.BPDA_CharacterInfo_C|GetSpellPassive (Variables|/Game/_Project/BP/BP_ApexCharacter.BP_ApexCharacter_C|GetCharacterInfo (Variables|Default|GetPlayer)))))

(event Input|EnhancedActionEvents|EnhancedInputActionIA_Ult
  (params (ActionValue :type Boolean) (ElapsedSeconds :type Float%20%28double-precision%29) (TriggeredSeconds :type Float%20%28double-precision%29) (InputAction :type Input%20Action%20Object%20Reference :default "/Game/_Project/Input/Actions/Spells/IA_Ult.IA_Ult"))
  (:Started
    (if (Default|IsActive (Variables|Default|GetUlt))
      (Default|Step (Variables|Default|GetUlt) (Variables|Default|GetPlayer))
      (elif (>= (Variables|Default|GetUltStack) (Variables|Default|GetUltStackMax))
        (Utilities|CastUlt)
        (else
          (Audio|PlaySound2D (Variables|Default|GetNoSpellSound) 1.0 1.0 0.0 0 0))))))

(fn CreateSpell
  (params (InputSpell :type BP%20Spell%20Class%20Reference))
  (bind _returnvalue (Game|SpawnActorfromClass InputSpell (Math|Transform|MakeTransform "0, 0, 0" "0, 0, 0" "1.000000,1.000000,1.000000") "Undefined" "MultiplyWithRoot" 0 0 0))
  (return _returnvalue))

(fn AddUltStack
  (if (>= (Variables|Default|GetUltStack) (Variables|Default|GetUltStackMax))
    (return true)
    (else
      (Math|Integer|IncrementInt (Variables|Default|GetUltStack)
        (:%20%20
          (Default|CallUltStackChange (Variables|Default|GetUltStack))
          (return false))))))