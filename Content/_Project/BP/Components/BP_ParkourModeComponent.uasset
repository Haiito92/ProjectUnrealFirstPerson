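; Actor component that runs parkour mode for BP_ApexCharacter, providing a run timer, speed readout and checkpoint respawn.
; On BeginPlay it creates the WD_ParkourTimerDisplay widget and stores the player's starting transform as the first checkpoint.
; Tick pushes speed in m/s and, while the timer is active, elapsed time to the widget.
; Exposed functions control the timer, update the checkpoint or teleport the player back with restored control rotation.
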(event Custom|CE_SetWaitingState
  (params (State :type Boolean))
  (Default|CESetWaitingState (Variables|Default|GetGUI) State))

(event EventBeginPlay
  (bind _asbp_apex_character (Utilities|Casting|CastToBP_ApexCharacter (Components|GetOwner)))
  (Variables|Default|SetPlayer _asbp_apex_character)
  (bind _returnvalue (UserInterface|CreateWidget "/Game/_Project/Widgets/Parkour/WD_ParkourTimerDisplay.WD_ParkourTimerDisplay_C" (Variables|/Game/_Project/BP/BP_ApexCharacter.BP_ApexCharacter_C|GetPlayerController _asbp_apex_character)))
  (bind _output_get (Variables|Default|SetGUI _returnvalue))
  (UserInterface|Viewport|AddtoPlayerScreen _output_get)
  (Checkpoint|CheckpointUpdate (Transformation|GetActorTransform (Variables|Default|GetPlayer))))

(event EventTick
  (params (DeltaSeconds :type Float%20%28single-precision%29))
  (CallFunction|UpdateSpeedDisplay)
  (if (Variables|Default|GetIsTimerActive)
    (bind _output_get (Variables|Default|SetTimer (+ DeltaSeconds (Variables|Default|GetTimer))))
    (Default|CEPassTimer (Variables|Default|GetGUI) _output_get)))

(fn StartTimer
  (Variables|Default|SetIsTimerActive true))

(fn ResetTimer
  (Variables|Default|SetTimer 0.0))

(fn StopTimer
  (Variables|Default|SetIsTimerActive false))

(fn RestartTimer
  (Timer|StopTimer) ; Just in case
  (Timer|ResetTimer)
  (Timer|StartTimer))

(fn UpdateSpeedDisplay
  (Default|CESetSpeedValue (Variables|Default|GetGUI) (Utilities|Text|ToText(String) (Utilities|String|Append (Utilities|String|ToString(Text) (Utilities|Text|ToText(Float) (/ (Math|Vector|VectorLength (Transformation|GetVelocity (Variables|Default|GetPlayer))) 1e+02) "HalfToEven" false true 1 324 2 2)) " m/s"))))

(fn ResettoLastCheckpoint
  (bind _player (Variables|Default|GetPlayer))
  (bind _lastcheckpointtransform (Variables|Default|GetLastCheckpointTransform))
  (Pawn|SetControlRotation (Variables|/Game/_Project/BP/BP_ApexCharacter.BP_ApexCharacter_C|GetPlayerController _player) (.Rotation (Math|Transform|BreakTransform _lastcheckpointtransform)))
  (Transformation|SetActorTransform _player _lastcheckpointtransform false true))

(fn CheckpointUpdate
  (params (CheckpointTransform :type Transform))
  (Variables|Default|SetLastCheckpointTransform CheckpointTransform))