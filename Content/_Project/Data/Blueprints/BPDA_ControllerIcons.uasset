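; Data asset that maps controller types to input key icons, used to look up button glyphs per controller.
; GetControllerIcons finds the icon set for a controller type in the ControllerIcons map.
; GetControllerIconForKey searches that set's nested map for a key and returns the icon with a Found flag.
; If either lookup fails, it returns a fixed fallback image with Found set to false.
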(fn GetControllerIcons
  (params (Controller%20Type :type EPlayerControllerType%20Enum :default "NewEnumerator0"))
  (bind _controllericons (Variables|Default|GetControllerIcons))
  (bind (_value _returnvalue) (Utilities|Map|Find _controllericons Controller%20Type))
  (return _value _returnvalue))

(fn GetControllerIconforKey
  (params (Controller%20Type :type EPlayerControllerType%20Enum :default "NewEnumerator0") (ControllerKey :type EControllerKey%20Enum :default "NewEnumerator0"))
  (bind (_icons _found) (CallFunction|GetControllerIcons Controller%20Type))
  (if (not _found)
    _
    (elif (not (.ReturnValue (Utilities|Map|Find (Utilities|Struct|BreakST_ControllerIcons _icons) ControllerKey)))
      _
      (else
        (return (.Value (Utilities|Map|Find (Utilities|Struct|BreakST_ControllerIcons _icons) ControllerKey)) true))))
  (return "/Game/_Project/Assets/Materials/FX/WindOrb/AdobeStock_439280145.AdobeStock_439280145" false))