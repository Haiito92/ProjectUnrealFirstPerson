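; BP_WallRide_5 is a wall ride building actor with three spinning propeller meshes.
; On BeginPlay, three RotatingMovement components are each bound to their own propeller component (Helice, Helice1, Helice2) so they rotate independently.
; The construction script applies the MeshDePasHelice mesh variable to the PasHelice component, letting the non-propeller part's mesh vary per instance.
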(event EventBeginPlay
  (Components|Movement|SetUpdatedComponent (Variables|Default|GetRotatingMovement) (Variables|Default|Gethelice))
  (Components|Movement|SetUpdatedComponent (Variables|Default|GetRotatingMovement1) (Variables|Default|Gethelice1))
  (Components|Movement|SetUpdatedComponent (Variables|Default|GetRotatingMovement2) (Variables|Default|Gethelice2)))

(event Collision|EventActorBeginOverlap
  (params (OtherActor :type Actor%20Object%20Reference)))

(event EventTick
  (params (DeltaSeconds :type Float%20%28single-precision%29)))

(fn ConstructionScript
  (Components|StaticMesh|SetStaticMesh (Variables|Default|Getpas%20helice) (Variables|Default|Getmesh%20de%20pas%20helice)))