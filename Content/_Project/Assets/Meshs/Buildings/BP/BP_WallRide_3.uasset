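; BP_WallRide_3 is a building Blueprint, named as a wall ride piece, with two spinning propellers (Helice) on a configurable static body.
; The construction script sets the non-propeller mesh (PasHelice) from a variable and applies a light material to its third material slot.
; On BeginPlay, each of two RotatingMovement components is bound to its own propeller, so they spin without any Tick logic.
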(event EventBeginPlay
  (Components|Movement|SetUpdatedComponent (Variables|Default|GetRotatingMovement) (Variables|Default|Gethelice))
  (Components|Movement|SetUpdatedComponent (Variables|Default|GetRotatingMovement1) (Variables|Default|Gethelice1)))

(event Collision|EventActorBeginOverlap
  (params (OtherActor :type Actor%20Object%20Reference)))

(event EventTick
  (params (DeltaSeconds :type Float%20%28single-precision%29)))

(fn ConstructionScript
  (bind _pas_helice (Variables|Default|Getpas%20helice))
  (Components|StaticMesh|SetStaticMesh _pas_helice (Variables|Default|Getmesh%20de%20pas%20helice))
  (Rendering|Material|SetMaterial _pas_helice 2 (Variables|Default|GetLightMat)))